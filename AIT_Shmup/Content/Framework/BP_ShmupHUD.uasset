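; BP_ShmupHUD is the shoot-'em-up HUD that owns the pause, level-up, weapon upgrade and main UI widgets.
; BeginPlay creates all four widgets once and stores their references, without adding any to the viewport.
; Level-up and weapon upgrade events pause the game and show their screens.
; The player pause event only shows the pause screen, and the main UI is not displayed here.
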(event Custom|PlayerLeveledUp
  (Game|SetGamePaused true)
  (UserInterface|Viewport|AddtoViewport (Variables|Default|GetLevelUpRef) 0))

(event Custom|WeaponUpgrade
  (Game|SetGamePaused true)
  (UserInterface|Viewport|AddtoViewport (Variables|Default|GetWeaponUpgradeRef) 0))

(event EventBeginPlay
  (bind _returnvalue (UserInterface|CreateWidget "/Game/UI/WBP_LevelUpScreen.WBP_LevelUpScreen_C" (Game|GetPlayerController 0)))
  (Variables|Default|SetLevelUpRef _returnvalue)
  (bind _returnvalue_2 (UserInterface|CreateWidget "/Game/UI/WBP_PauseScreen.WBP_PauseScreen_C" (Game|GetPlayerController 0)))
  (Variables|Default|SetPauseRef _returnvalue_2)
  (bind _returnvalue_3 (UserInterface|CreateWidget "/Game/UI/WBP_HUDUI.WBP_HUDUI_C" (Game|GetPlayerController 0)))
  (Variables|Default|SetUI%20Ref _returnvalue_3)
  (bind _returnvalue_4 (UserInterface|CreateWidget "/Game/UI/WBP_WeaponUpgradeScreen.WBP_WeaponUpgradeScreen_C"))
  (Variables|Default|SetWeaponUpgradeRef _returnvalue_4))

(event EventPlayerPause
  (UserInterface|Viewport|AddtoViewport (Variables|Default|GetPauseRef) 0))

(fn ConstructionScript)