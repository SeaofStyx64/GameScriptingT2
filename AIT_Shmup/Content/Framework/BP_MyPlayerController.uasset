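; BP_MyPlayerController is the player controller for a shoot-'em-up, handling pause input, the mouse cursor and the player's life count.
; Escape casts the HUD to BP_ShmupHUD, sends it the pause message, then triggers PlayerPauses on its PauseRef.
; BeginPlay shows a crosshair cursor.
; The ChangePlayerLives event adds the given amount to PlayerLives, with no clamping or game-over check here.
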(event EventBeginPlay
  (Variables|Default|SetbShowMouseCursor true)
  (Variables|Default|SetCurrentMouseCursor "Crosshairs"))

(event EventChangePlayerLives
  (params (LivesToAdd :type Integer))
  (Variables|Default|SetPlayerLives (+ (Variables|Default|GetPlayerLives) LivesToAdd)))

(event Input|KeyboardEvents|Escape
  (params (Key :type Key%20Structure :default "None"))
  (bind _returnvalue (HUD|GetHUD))
  (:Pressed
    (bind _asbp_shmup_hud (Utilities|Casting|CastToBP_ShmupHUD _returnvalue))
    (Class|BPISpaceshipFunctions|PlayerPause(Message) _returnvalue)
    (Default|PlayerPauses (Variables|/Game/Framework/BP_ShmupHUD.BP_ShmupHUD_C|GetPauseRef _asbp_shmup_hud))))

(fn ConstructionScript)