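; BP_Indicator_Revive is a short-lived effect actor that displays a "REVIVED" text indicator in the world.
; On BeginPlay it sets the text and colour on the WBP_Indicator inside its DamageNumber widget component.
; A timeline then drives the component's scale and tint flash, and the actor destroys itself when the timeline finishes.
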(event EventBeginPlay
  (bind _aswbp_indicator (Utilities|Casting|CastToWBP_Indicator (UserInterface|GetUserWidgetObject (Variables|Default|GetDamageNumber))))
  (Default|ChangeValue _aswbp_indicator "REVIVED")
  (Appearance|SetColorandOpacity _aswbp_indicator (Variables|Default|GetTextColour) :!class /Script/UMG.UserWidget)
  (bind (_direction _scalingsingle _flashtrack) (Timeline|Timeline Play)
    (:Update
      (Transformation|SetRelativeScale3D (Variables|Default|GetDamageNumber) (Math|Vector|MakeVector _scalingsingle _scalingsingle _scalingsingle))
      (Class|WidgetComponent|SetTintColorandOpacity (Variables|Default|GetDamageNumber) (Math|Conversions|ToLinearColor(Float) _flashtrack)))
    (:Finished
      (Actor|DestroyActor))))

(fn ConstructionScript)