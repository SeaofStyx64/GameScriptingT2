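; BP_Indicator is a short-lived actor that shows a number, likely damage, through a WBP_Indicator widget on its DamageNumber component.
; The ChangeNumber event passes a value to that widget and tints it with TextColour.
; On BeginPlay, a timeline animates the component's uniform scale and destroys the actor when it finishes.
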(event Custom|ChangeNumber
  (params (NumberChangeTo :type Text))
  (bind _aswbp_indicator (Utilities|Casting|CastToWBP_Indicator (UserInterface|GetUserWidgetObject (Variables|Default|GetDamageNumber))))
  (Default|ChangeValue _aswbp_indicator NumberChangeTo)
  (Appearance|SetColorandOpacity _aswbp_indicator (Variables|Default|GetTextColour) :!class /Script/UMG.UserWidget))

(event EventBeginPlay
  (bind _scalingsingle (Timeline|Timeline Play)
    (:Update
      (Transformation|SetRelativeScale3D (Variables|Default|GetDamageNumber) (Math|Vector|MakeVector _scalingsingle _scalingsingle _scalingsingle)))
    (:Finished
      (Actor|DestroyActor))))

(event Collision|EventActorBeginOverlap
  (params (OtherActor :type Actor%20Object%20Reference)))

(event EventTick
  (params (DeltaSeconds :type Float%20%28single-precision%29)))

(fn ConstructionScript)