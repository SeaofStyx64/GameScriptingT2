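; Enemy spawner actor that endlessly spawns random enemy classes from a pool after play begins.
; A self-requeuing timer fires at a random interval, spawning an enemy and scheduling the next.
; Each spawn samples random points on start and end splines, placing the enemy at the first, facing the second.
; All randomness draws from one random stream seeded with a fixed value, so the sequence is repeatable.
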(event Custom|SpawnEnemy
  (bind (_startlocation _endlocation) (CallFunction|GetStart&EndLocation))
  (bind _output_get (Variables|Default|SetSpawnTrans (Math|Transform|MakeTransform _startlocation (Math|Rotator|FindLookatRotation _startlocation _endlocation) "1.000000,1.000000,1.000000")))
  (Game|SpawnActorfromClass (.OutItem (Utilities|Array|RandomFromStream (Variables|Default|GetEnemyClassPool) (Variables|Default|GetRandomStream))) _output_get "AlwaysSpawn" "MultiplyWithRoot" 0 0)
  (CallFunction|QueueSpawn))

(event Custom|QueueSpawn
  (bind _returnvalue (Utilities|Time|SetTimerbyEvent (delegate Custom|SpawnEnemy) (Math|Random|RandomFloatinRangefromStream (Variables|Default|GetRandomStream) 0.5 2.0) false true))
  (Variables|Default|SetEnemySpawnRate _returnvalue))

(event Collision|EventActorBeginOverlap
  (params (OtherActor :type Actor%20Object%20Reference)))

(event EventTick
  (params (DeltaSeconds :type Float%20%28single-precision%29)))

(event EventBeginPlay
  (Math|Random|SetRandomStreamSeed (Variables|Default|GetRandomStream) 0)
  (CallFunction|QueueSpawn))

(fn ConstructionScript)

(fn GetStart&EndLocation
  (bind _randomstream (Variables|Default|GetRandomStream))
  (bind _returnvalue (Math|Random|RandomFloatfromStream _randomstream))
  (return (Spline|GetLocationatTime (Variables|Default|GetStartLocation) _returnvalue "World" false) (Spline|GetLocationatTime (Variables|Default|GetEndLocation) _returnvalue "World" false)))