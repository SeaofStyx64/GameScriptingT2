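; Player ship pawn variant that overrides weapon firing to launch star bullets (BP_PBullet_Star).
; When firing is allowed, it plays a randomly pitched laser sound and spawns a bullet at the middle fire point.
; Higher weapon tiers raise the bullet's hits-before-destroy count, then a fire-rate-scaled timer calls FireCoolDown.
; Any homing implied by the asset name is not implemented in this graph.
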(event EventBeginPlay
  (|CallParentFunction) ; This node is disabled and will not be called.\nDrag off pins to build functionality.
)

(event Collision|EventActorBeginOverlap
  (params (OtherActor :type Actor%20Object%20Reference)))

(event EventTick
  (params (DeltaSeconds :type Float%20%28single-precision%29))
  (|CallParentFunction DeltaSeconds) ; This node is disabled and will not be called.\nDrag off pins to build functionality.
)

(event EventFireWeapon
  (bind _firespawnpointmid (Variables|Default|GetFireSpawnPointMid))
  (bind _returnvalue (Transformation|GetWorldTransform _firespawnpointmid))
  (if (Variables|Default|GetCanFireWeapon)
    (Variables|Default|SetIsFiringWeapon true)
    (Audio|PlaySound2D "/Game/SoundFX/Laser1.Laser1" 0.2 (Math|Random|RandomFloatinRange 0.5 1.0) 0.0 0 0)
    (bind _returnvalue_2 (Game|SpawnActorfromClass "/Game/Blueprints/BulletsAndSummons/BP_PBullet_Star.BP_PBullet_Star_C" (Math|Transform|MakeTransform (.location _returnvalue) (.rotation _returnvalue) "1.000000,1.000000,1.000000") "AlwaysSpawn" "MultiplyWithRoot" 0 0))
    (switch int (Variables|Default|GetWeaponTier)
      (:0
        _)
      (:1
        (Variables|/Game/Blueprints/BulletsAndSummons/BP_PBullet_Star.BP_PBullet_Star_C|SetHitsTillDestroy _returnvalue_2 1))
      (:2
        (Variables|/Game/Blueprints/BulletsAndSummons/BP_PBullet_Star.BP_PBullet_Star_C|SetHitsTillDestroy _returnvalue_2 2)))
    (Variables|Default|SetCanFireWeapon false)
    (bind _newfirerate (CallFunction|FirerateCalculation 0.8))
    (Utilities|Time|SetTimerbyFunctionName 0 "FireCoolDown" _newfirerate)))

(fn ConstructionScript
  (|CallParentFunction))