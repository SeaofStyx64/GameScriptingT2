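; Player ship pawn variant whose weapon fires a shotgun-style fan of BP_PBullet_TripleShot projectiles.
; FireWeapon plays a randomly pitched laser sound, then uses WeaponTier to set base fire rate, bullet count and starting angle.
; A loop spawns bullets from the actor's transform at evenly stepped yaw offsets, then a FireCoolDown timer, timed by FirerateCalculation, follows.
; Older spawn nodes using FireSpawnPointMid remain disconnected.
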(event EventFireWeapon
  (bind _returnvalue (Transformation|GetActorTransform))
  (if (Variables|Default|GetCanFireWeapon)
    (Variables|Default|SetIsFiringWeapon true)
    (Audio|PlaySound2D "/Game/SoundFX/Laser1.Laser1" 0.2 (Math|Random|RandomFloatinRange 0.1 0.4) 0.0 0 0)
    (switch int (Variables|Default|GetWeaponTier)
      (:Default
        (Variables|Default|SetBaseFirerate 1.2 :!label _label)
        (Variables|Default|SetBulletCount 3)
        (Variables|Default|SetBulletAngle -1e+01))
      (:0
        (goto _label))
      (:1
        (Variables|Default|SetBaseFirerate 1.1)
        (Variables|Default|SetBulletCount 5)
        (Variables|Default|SetBulletAngle -2e+01))
      (:2
        (Variables|Default|SetBaseFirerate 1.0)
        (Variables|Default|SetBulletCount 7)
        (Variables|Default|SetBulletAngle -3e+01)))
    (for _index (range 1 (Variables|Default|GetBulletCount))
      (Game|SpawnActorfromClass "/Game/Blueprints/BulletsAndSummons/BP_PBullet_TripleShot.BP_PBullet_TripleShot_C" (Math|Transform|MakeTransform (.location _returnvalue) (Math|Rotator|MakeRotator (.roll (.rotation _returnvalue)) (.pitch (.rotation _returnvalue)) (+ (.yaw (.rotation _returnvalue)) (Variables|Default|GetBulletAngle))) "1.000000,1.000000,1.000000") "AlwaysSpawn" "MultiplyWithRoot" 0 0)
      (Variables|Default|SetBulletAngle (+ (Variables|Default|GetBulletAngle) 1e+01)))
    (Variables|Default|SetCanFireWeapon false)
    (bind _newfirerate (CallFunction|FirerateCalculation (Variables|Default|GetBaseFirerate)))
    (Utilities|Time|SetTimerbyFunctionName 0 "FireCoolDown" _newfirerate)))

(fn ConstructionScript
  (|CallParentFunction))