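; Player ship pawn for a shoot 'em up: moves through Enhanced Input, turns toward the mouse cursor and banks when strafing.
; Bullet and enemy overlaps feed dodge, defence, forcefield and invincibility-frame logic, leading to lives-based revive or death.
; Upgrade and pickup events alter stats, heal, score or attach turrets, sawguards and forcefields, updating the HUD on health changes.
; Firing is forwarded as an interface message, with a helper computing the clamped fire interval.
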(event OnComponentBeginOverlap(Box)
  (params (OverlappedComponent :type Primitive%20Component%20Object%20Reference) (OtherActor :type Actor%20Object%20Reference) (OtherComp :type Primitive%20Component%20Object%20Reference) (OtherBodyIndex :type Integer) (bFromSweep :type Boolean) (SweepResult :type Hit%20Result%20Structure%20%28by%20ref%29))
  ;[0.15 0.15 0.15 0.5] When Contacting Other Object
  (if (not (Variables|Default|GetIsInvincible))
    (if (Variables|Default|GetForcefieldUp)
      (Variables|Default|SetForcefieldUp false)
      (bind _returnvalue (Actor|GetActorOfClass "/Game/Blueprints/BP_Forcefield.BP_Forcefield_C"))
      (Actor|DestroyActor _returnvalue)
      (else
        (bind _asbp_base_enemy_bullet (Utilities|Casting|CastToBP_BaseEnemyBullet OtherActor)
          (:then
            (CallFunction|ApplyDamagetoPlayer (Variables|/Game/Blueprints/BulletsAndSummons/BP_BaseEnemyBullet.BP_BaseEnemyBullet_C|GetDamage _asbp_base_enemy_bullet)))
          (:CastFailed
            (bind _asbp_enemy_base (Utilities|Casting|CastToBP_Enemy_Base OtherActor))
            (CallFunction|ApplyDamagetoPlayer (Variables|/Game/Blueprints/Enemies/BP_Enemy_Base.BP_Enemy_Base_C|GetContactDamage _asbp_enemy_base))))
        (Variables|Default|SetIsInvincible true)
        (Utilities|Time|SetTimerbyEvent (delegate Custom|NoMoreIFrames) 0.5)))))

(event Custom|ApplyDamageToPlayer
  (params (DamageTaken :type Float%20%28double-precision%29))
  (bind _upgradedefence (Variables|Default|GetUpgradeDefence))
  (bind _returnvalue (* DamageTaken _upgradedefence))
  (bind _returnvalue_2 (- DamageTaken _returnvalue))
  ;[0.15 0.15 0.15 0.5] Applying Damage Taken When Hit
  (if (<= (Math|Random|RandomFloatinRange 0.0 1.0) (/ (Variables|Default|GetDodgeChance) 1e+02))
    (CallFunction|Dodged)
    (else
      (Variables|Default|SetHealth (- (Variables|Default|GetHealth) _returnvalue_2))
      (bind _returnvalue_3 (Game|SpawnActorfromClass "/Game/Blueprints/Indicators/BP_Indicator_Damage.BP_Indicator_Damage_C" (Math|Transform|MakeTransform (Transformation|GetActorLocation) "0, 0, 0" "1.000000,1.000000,1.000000") "AlwaysSpawn" "MultiplyWithRoot" 0 0))
      (Default|ChangeNumber _returnvalue_3 (Utilities|Text|ToText(Float) _returnvalue_2 "HalfToEven"))
      (if (<= (Variables|Default|GetHealth) 0.0)
        _
        (else
          (CallFunction|DamageOverlay)))
      (Audio|PlaySound2D "/Game/SoundFX/PlayerHit.PlayerHit" 1.0 1.0 0.0 0 0)
      (bind _asbp_shmup_hud (Utilities|Casting|CastToBP_ShmupHUD (HUD|GetHUD (Game|GetPlayerController 0))))
      (Default|HealthChanges (Variables|/Game/Framework/BP_ShmupHUD.BP_ShmupHUD_C|GetUI%20Ref _asbp_shmup_hud) (/ (Variables|Default|GetHealth) (Variables|Default|GetMaxHealth)))
      (if (<= (Variables|Default|GetHealth) 0.0)
        (CallFunction|PlayerDies)))))

(event Custom|DamageOverlay
  ;[0.15 0.15 0.15 0.5] Visual Effect When Being Hit
  (Rendering|Material|SetOverlayMaterial (Variables|Default|GetShipModel) "/Game/Materials/M_DamageOverlay_Player.M_DamageOverlay_Player" :!class /Script/Engine.MeshComponent)
  (Utilities|FlowControl|Delay 0.2)
  (Rendering|Material|SetOverlayMaterial (Variables|Default|GetShipModel) "/Game/Materials/M_OutlinePlayer.M_OutlinePlayer" :!class /Script/Engine.MeshComponent))

(event Custom|Regeneration
  (bind _upgraderegen (Variables|Default|GetUpgradeRegen))
  ;[0.15 0.15 0.15 0.5] Regeneration
  (if (< (Variables|Default|GetHealth) (Variables|Default|GetMaxHealth))
    (Utilities|FlowControl|Delay 5.0)
    (Variables|Default|SetHealth (+ (Variables|Default|GetHealth) _upgraderegen))
    (bind _returnvalue (Game|SpawnActorfromClass "/Game/Blueprints/Indicators/BP_Indicator_Regen.BP_Indicator_Regen_C" (Math|Transform|MakeTransform (Transformation|GetActorLocation) "0, 0, 0" "1.000000,1.000000,1.000000") "AlwaysSpawn" "MultiplyWithRoot" 0 0))
    (Default|ChangeNumber _returnvalue (Utilities|Text|ToText(Float) _upgraderegen "HalfToEven"))
    (bind _asbp_shmup_hud (Utilities|Casting|CastToBP_ShmupHUD (HUD|GetHUD (Game|GetPlayerController 0))))
    (Default|HealthChanges (Variables|/Game/Framework/BP_ShmupHUD.BP_ShmupHUD_C|GetUI%20Ref _asbp_shmup_hud) (/ (Variables|Default|GetHealth) (Variables|Default|GetMaxHealth)))
    (Rendering|Material|SetOverlayMaterial (Variables|Default|GetShipModel) "/Game/Materials/M_RegenOverlay.M_RegenOverlay" :!class /Script/Engine.MeshComponent)
    (Utilities|FlowControl|Delay 0.1)
    (Rendering|Material|SetOverlayMaterial (Variables|Default|GetShipModel) "/Game/Materials/M_OutlinePlayer.M_OutlinePlayer" :!class /Script/Engine.MeshComponent)))

(event Custom|HealPlayer
  (params (HealthHealed :type Float%20%28double-precision%29) (Revive? :type Boolean))
  ;[0.15 0.15 0.15 0.5] Healing
  (bind _returnvalue (Game|SpawnActorfromClass "/Game/Blueprints/Indicators/BP_Indicator_Health.BP_Indicator_Health_C" (Math|Transform|MakeTransform (Transformation|GetActorLocation) "0, 0, 0" "1.000000,1.000000,1.000000") "AlwaysSpawn" "MultiplyWithRoot" 0 0))
  (Default|ChangeNumber _returnvalue (Utilities|Text|ToText(Float) HealthHealed "HalfToEven"))
  (if (>= (+ (Variables|Default|GetHealth) HealthHealed) (Variables|Default|GetMaxHealth))
    (Variables|Default|SetHealth (Variables|Default|GetMaxHealth))
    (else
      (Variables|Default|SetHealth (+ (Variables|Default|GetHealth) HealthHealed))))
  (bind _asbp_shmup_hud (Utilities|Casting|CastToBP_ShmupHUD (HUD|GetHUD (Game|GetPlayerController 0))))
  (Default|HealthChanges (Variables|/Game/Framework/BP_ShmupHUD.BP_ShmupHUD_C|GetUI%20Ref _asbp_shmup_hud) (/ (Variables|Default|GetHealth) (Variables|Default|GetMaxHealth)))
  (Audio|PlaySound2D "/Game/SoundFX/PlayerHeal.PlayerHeal" 0.3 1.0 0.0 0 0)
  (if (not Revive?)
    (Rendering|Material|SetOverlayMaterial (Variables|Default|GetShipModel) "/Game/Materials/M_HealOverlay.M_HealOverlay" :!class /Script/Engine.MeshComponent)
    (Utilities|FlowControl|Delay 0.2)
    (Rendering|Material|SetOverlayMaterial (Variables|Default|GetShipModel) "/Game/Materials/M_OutlinePlayer.M_OutlinePlayer" :!class /Script/Engine.MeshComponent)))

(event Custom|RevivePlayer
  (bind _shipmodel (Variables|Default|GetShipModel))
  ;[0.15 0.15 0.15 0.5] Revive Sequence
  (Rendering|Material|SetOverlayMaterial _shipmodel "/Game/Materials/M_ReviveOverlay.M_ReviveOverlay" :!class /Script/Engine.MeshComponent)
  (CallFunction|HealPlayer (Variables|Default|GetMaxHealth) true)
  (Utilities|FlowControl|Delay 1.0)
  (Rendering|Material|SetOverlayMaterial _shipmodel "/Game/Materials/M_OutlinePlayer.M_OutlinePlayer" :!class /Script/Engine.MeshComponent))

(event Custom|BecomeTitan
  ;[0.15 0.15 0.15 0.5] Titan Upgrade
  (bind _output_get (Variables|Default|SetCurrentScale (+ (Variables|Default|GetCurrentScale) "0.500000,0.500000,0.500000")))
  (Transformation|SetActorRelativeScale3D _output_get)
  (Variables|Default|SetUpgradeDamage (+ (Variables|Default|GetUpgradeDamage) 1.75))
  (bind _output_get_2 (Variables|Default|SetMaxHealth (* (Variables|Default|GetMaxHealth) 2.0)))
  (CallFunction|HealPlayer (/ _output_get_2 2.0) false))

(event Custom|BecomeGlass
  ;[0.15 0.15 0.15 0.5] Glass Cannon Upgrade
  (Variables|Default|SetMaxHealth (/ (Variables|Default|GetMaxHealth) 4.0))
  (Variables|Default|SetHealth (/ (Variables|Default|GetHealth) 4.0))
  (Variables|Default|SetUpgradeDamage (+ (Variables|Default|GetUpgradeDamage) 3.0))
  (bind _asbp_shmup_hud (Utilities|Casting|CastToBP_ShmupHUD (HUD|GetHUD (Game|GetPlayerController 0))))
  (Default|HealthChanges (Variables|/Game/Framework/BP_ShmupHUD.BP_ShmupHUD_C|GetUI%20Ref _asbp_shmup_hud) (/ (Variables|Default|GetHealth) (Variables|Default|GetMaxHealth))))

(event Custom|FireCoolDown
  ;[0.15 0.15 0.15 0.5] Shoot when click
  (Variables|Default|SetCanFireWeapon true))

(event Custom|SawguardSpawn
  (params (2%20Saws? :type Boolean))
  (bind _centrepoint (Variables|Default|GetCentrePoint))
  (bind _returnvalue (Transformation|GetRelativeTransform _centrepoint))
  ;[0.15 0.15 0.15 0.5] Sawguard Upgrade logic
  (if 2%20Saws?
    (bind _returnvalue_2 (Game|SpawnActorfromClass "/Game/Blueprints/BulletsAndSummons/BP_Sawguard2.BP_Sawguard2_C" _returnvalue "AlwaysSpawn" "MultiplyWithRoot" 0 0))
    (Transformation|AttachComponentToComponent _returnvalue_2 (Variables|Default|GetCentrePoint) "None" "KeepRelative" "KeepWorld" "KeepRelative" true)
    (Actor|DestroyActor (stale _returnvalue_3))
    (else
      (bind _returnvalue_3 (Game|SpawnActorfromClass "/Game/Blueprints/BulletsAndSummons/BP_Sawguard1.BP_Sawguard1_C" _returnvalue "AlwaysSpawn" "MultiplyWithRoot" 0 0))
      (Transformation|AttachComponentToComponent _returnvalue_3 (Variables|Default|GetCentrePoint) "None" "KeepRelative" "KeepWorld" "KeepRelative" true))))

(event Custom|SpawnTurret
  (params (2ndTurret? :type Boolean))
  ;[0.15 0.15 0.15 0.5] Summon Turrets
  (if 2ndTurret?
    (bind _returnvalue (Game|SpawnActorfromClass "/Game/Blueprints/BulletsAndSummons/BP_WingTurret.BP_WingTurret_C" (Transformation|GetRelativeTransform (Variables|Default|GetTurretSpawnL)) "AlwaysSpawn" "MultiplyWithRoot" 0 0))
    (Transformation|AttachComponentToComponent _returnvalue (Variables|Default|GetTurretSpawnL) "None" "KeepRelative" "KeepRelative" "KeepRelative" true)
    (else
      (bind _returnvalue_2 (Game|SpawnActorfromClass "/Game/Blueprints/BulletsAndSummons/BP_WingTurret.BP_WingTurret_C" (Transformation|GetRelativeTransform (Variables|Default|GetTurretSpawnR)) "AlwaysSpawn" "MultiplyWithRoot" 0 0))
      (Transformation|AttachComponentToComponent _returnvalue_2 (Variables|Default|GetTurretSpawnR) "None" "KeepRelative" "KeepRelative" "KeepRelative" true))))

(event Custom|SetMouseTargetLocation
  (bind _returnvalue (Game|GetPlayerController 0))
  (bind _hitresult (Game|Player|GetHitResultUnderCursorbyChannel _returnvalue "TraceTypeQuery1" true))
  (bind _location (Collision|BreakHitResult _hitresult))
  ;[0.15 0.15 0.15 0.5] Aim at Mouse
  (Transformation|SetWorldLocation (Variables|Default|GetMouseLocation) _location false false)
  (Transformation|SetActorRotation (Math|Rotator|MakeRotator 0.0 0.0 (.yaw (Math|Rotator|Lerp(Rotator) (Math|Rotator|MakeRotator 0.0 0.0 (.yaw (Transformation|GetActorRotation))) (Math|Rotator|MakeRotator 0.0 0.0 (.yaw (Math|Rotator|FindLookatRotation (Transformation|GetActorLocation) _location))) 0.15 true)))))

(event Custom|NoMoreIFrames
  ;[0.15 0.15 0.15 0.5] When Contacting Other Object
  (Variables|Default|SetIsInvincible false))

(event Custom|ItemPickup
  (params (PickupID :type Integer))
  ;[0.15 0.15 0.15 0.5] Pickup Manager
  (switch int PickupID
    (:0
      (CallFunction|HealPlayer 3e+01 false))
    (:1
      (bind _asbp_shmup_hud (Utilities|Casting|CastToBP_ShmupHUD (HUD|GetHUD (Game|GetPlayerController 0))))
      (Default|IncreaseScore (Variables|/Game/Framework/BP_ShmupHUD.BP_ShmupHUD_C|GetUI%20Ref _asbp_shmup_hud) 5e+01))
    (:2
      (Variables|Default|SetForcefieldUp true)
      (bind _returnvalue (Game|SpawnActorfromClass "/Game/Blueprints/BP_Forcefield.BP_Forcefield_C" (Math|Transform|MakeTransform (Transformation|GetWorldLocation (Variables|Default|GetCentrePoint)) "0, 0, 0" "1.000000,1.000000,1.000000") "AlwaysSpawn" "MultiplyWithRoot" 0 0))
      (Transformation|AttachComponentToComponent _returnvalue (Variables|Default|GetCentrePoint) "None" "KeepWorld" "KeepWorld" "KeepWorld" true))))

(event Custom|PlayerDies
  ;[0.15 0.15 0.15 0.5] Player Death Sequence
  (bind _asbp_my_player_controller (Utilities|Casting|CastToBP_MyPlayerController (Game|GetPlayerController 0)))
  (Variables|/Game/Framework/BP_MyPlayerController.BP_MyPlayerController_C|SetPlayerLives _asbp_my_player_controller (- (Variables|/Game/Framework/BP_MyPlayerController.BP_MyPlayerController_C|GetPlayerLives _asbp_my_player_controller) 1))
  (if (== (Variables|/Game/Framework/BP_MyPlayerController.BP_MyPlayerController_C|GetPlayerLives _asbp_my_player_controller) 0)
    (Audio|PlaySound2D "/Game/SoundFX/Explosion1.Explosion1" 1.0 (Math|Random|RandomFloatinRange 0.5 1.0) 0.0 0 0)
    (Game|SpawnActorfromClass "/Game/Particles/BP_PlayerDeathParticle.BP_PlayerDeathParticle_C" (Transformation|GetActorTransform) "AlwaysSpawn" "MultiplyWithRoot" 0 0)
    (Input|DisableInput (Game|GetPlayerController 0))
    (Class|BPISpaceshipFunctions|PlayerDeath(Message) (Game|GetPlayerController 0))
    (Actor|DestroyActor)
    (else
      (CallFunction|RevivePLayer))))

(event Custom|IncreaseSpeed
  (bind _floatingpawnmovement (Variables|Default|GetFloatingPawnMovement))
  ;[0.15 0.15 0.15 0.5] Increase Speed when upgrade is chosen
  (Variables|/Script/Engine.FloatingPawnMovement|SetMaxSpeed _floatingpawnmovement (+ (Variables|/Script/Engine.FloatingPawnMovement|GetMaxSpeed _floatingpawnmovement) (Variables|Default|GetUpgradeSpeed))))

(event Custom|Dodged
  ;[0.15 0.15 0.15 0.5] Visual Effect when dodging damage
  (Rendering|Material|SetOverlayMaterial (Variables|Default|GetShipModel) "/Game/Materials/M_DodgeOverlay.M_DodgeOverlay" :!class /Script/Engine.MeshComponent)
  (Utilities|FlowControl|Delay 0.2)
  (Rendering|Material|SetOverlayMaterial (Variables|Default|GetShipModel) "/Game/Materials/M_OutlinePlayer.M_OutlinePlayer" :!class /Script/Engine.MeshComponent))

(event Input|EnhancedActionEvents|EnhancedInputActionIA_Forward
  (params (ActionValue :type Boolean) (ElapsedSeconds :type Float%20%28double-precision%29) (TriggeredSeconds :type Float%20%28double-precision%29) (InputAction :type Input%20Action%20Object%20Reference :default "/Game/Data/IA_Forward.IA_Forward"))
  ;[0.15 0.15 0.15 0.5] Movement
  (Class|PawnMovementComponent|AddInputVector (Variables|Default|GetFloatingPawnMovement) "1.000000,0.000000,0.000000" false))

(event Input|EnhancedActionEvents|EnhancedInputActionIA_Right
  (params (ActionValue :type Boolean) (ElapsedSeconds :type Float%20%28double-precision%29) (TriggeredSeconds :type Float%20%28double-precision%29) (InputAction :type Input%20Action%20Object%20Reference :default "/Game/Data/IA_Right.IA_Right"))
  ;[0.15 0.15 0.15 0.5] Movement
  (Class|PawnMovementComponent|AddInputVector (Variables|Default|GetFloatingPawnMovement) "0.000000,1.000000,0.000000" false))

(event Input|EnhancedActionEvents|EnhancedInputActionIA_PrimaryShoot
  (params (ActionValue :type Boolean) (ElapsedSeconds :type Float%20%28double-precision%29) (TriggeredSeconds :type Float%20%28double-precision%29) (InputAction :type Input%20Action%20Object%20Reference :default "/Game/Data/IA_PrimaryShoot.IA_PrimaryShoot"))
  ;[0.15 0.15 0.15 0.5] Shoot when click
  (:Triggered
    (Class|BPISpaceshipFunctions|FireWeapon(Message) (Game|Player|GetPlayerPawn 0)))
  (:Completed
    (Variables|Default|SetIsFiringWeapon false)))

(event Input|EnhancedActionEvents|EnhancedInputActionIA_Left
  (params (ActionValue :type Boolean) (ElapsedSeconds :type Float%20%28double-precision%29) (TriggeredSeconds :type Float%20%28double-precision%29) (InputAction :type Input%20Action%20Object%20Reference :default "/Game/Data/IA_Left.IA_Left"))
  ;[0.15 0.15 0.15 0.5] Movement
  (Class|PawnMovementComponent|AddInputVector (Variables|Default|GetFloatingPawnMovement) "0.000000,-1.000000,0.000000" false))

(event Input|EnhancedActionEvents|EnhancedInputActionIA_Backwards
  (params (ActionValue :type Boolean) (ElapsedSeconds :type Float%20%28double-precision%29) (TriggeredSeconds :type Float%20%28double-precision%29) (InputAction :type Input%20Action%20Object%20Reference :default "/Game/Data/IA_Backwards.IA_Backwards"))
  ;[0.15 0.15 0.15 0.5] Movement
  (Class|PawnMovementComponent|AddInputVector (Variables|Default|GetFloatingPawnMovement) "-1.000000,0.000000,0.000000" false))

(event EventBeginPlay
  ;[0.15 0.15 0.15 0.5] Add Mapping at Start
  (Variables|Default|SetHealth (Variables|Default|GetMaxHealth))
  (bind _asplayer_controller (Utilities|Casting|CastToPlayerController (Pawn|GetController)))
  (Input|AddMappingContext (PlayerController|LocalPlayerSubsystems|GetEnhancedInputLocalPlayerSubsystem _asplayer_controller) "/Game/Data/PlayerControlMapping.PlayerControlMapping" 0 "(bIgnoreAllPressedKeysUntilRelease=True,bForceImmediately=False,bNotifyUserSettings=False)"))

(event EventTick
  (params (DeltaSeconds :type Float%20%28single-precision%29))
  (bind _returnvalue (Input|EnhancedActionValues|GetIA_Right))
  (bind _returnvalue_2 (Input|EnhancedActionValues|GetIA_Left))
  (bind _returnvalue_3 (Math|Float|SelectFloat -1.0 0.0 _returnvalue))
  (bind _returnvalue_4 (Math|Float|SelectFloat 1.0 _returnvalue_3 _returnvalue_2))
  (if (Variables|Default|GetUpgradeRegenUnlocked)
    (CallFunction|Regeneration))
  ;[0.15 0.15 0.15 0.5] Plane Roll
  (CallFunction|SetMouseTargetLocation)
  (Variables|Default|SetTargetBankAngle _returnvalue_4)
  (Variables|Default|SetCurrentBankAngle (Math|Interpolation|FInterpTo (Variables|Default|GetCurrentBankAngle) _returnvalue_4 DeltaSeconds 8.0))
  (Transformation|SetRelativeRotation (Variables|Default|GetShipModel) (Math|Rotator|MakeRotator (* (Variables|Default|GetMaxBankAngle) (Variables|Default|GetCurrentBankAngle)) 0.0 1.8e+02) false false))

(fn ConstructionScript)

(fn FirerateCalculation
  (params (BulletBaseFirerate :type Float%20%28double-precision%29))
  (bind _upgradefirerate (Variables|Default|GetUpgradeFirerate))
  (bind _returnvalue (Math|Float|Power 0.9 _upgradefirerate))
  (bind _returnvalue_2 (* BulletBaseFirerate _returnvalue))
  (if (<= _returnvalue_2 0.05)
    (return 0.05)
    (else
      (return _returnvalue_2))))