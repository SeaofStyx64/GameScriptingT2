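; Player ship pawn variant whose weapon is a melee sword, built on a parent ship Blueprint.
; FireWeapon, gated by CanFireWeapon, plays a pitch-randomized charge-up sound and spawns a sword bullet actor attached to the middle fire point so it follows the ship.
; WeaponTier selects the sword class and base fire rate, defaulting to the first tier.
; FirerateCalculation turns that rate into the delay for the FireCoolDown timer.
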(event EventFireWeapon
  (bind _firespawnpointmid (Variables|Default|GetFireSpawnPointMid))
  (bind _firespawnpointmid_2 (Variables|Default|GetFireSpawnPointMid))
  (bind _returnvalue (Transformation|GetWorldTransform _firespawnpointmid))
  (if (Variables|Default|GetCanFireWeapon)
    (Variables|Default|SetIsFiringWeapon true)
    (Audio|PlaySound2D "/Game/SoundFX/Chargeup.Chargeup" 1.0 (Math|Random|RandomFloatinRange 0.8 1.0) 0.0 0 0)
    (Variables|Default|SetCanFireWeapon false)
    (switch int (Variables|Default|GetWeaponTier)
      (:Default
        (bind _returnvalue_2 (Game|SpawnActorfromClass "/Game/Blueprints/BulletsAndSummons/BP_PBullet_SwordTier1.BP_PBullet_SwordTier1_C" (Math|Transform|MakeTransform (.location _returnvalue) (.rotation _returnvalue) "1.000000,1.000000,1.000000") "AlwaysSpawn" "MultiplyWithRoot" 0 0 :!label _label))
        (Transformation|AttachComponentToComponent _returnvalue_2 _firespawnpointmid_2 "None" "KeepWorld" "KeepWorld" "KeepWorld" true)
        (Variables|Default|SetBaseFirerate 0.9))
      (:0
        (goto _label))
      (:1
        (bind _returnvalue_3 (Game|SpawnActorfromClass "/Game/Blueprints/BulletsAndSummons/BP_PBullet_SwordTier2.BP_PBullet_SwordTier2_C" (Math|Transform|MakeTransform (.location _returnvalue) (.rotation _returnvalue) "1.000000,1.000000,1.000000") "AlwaysSpawn" "MultiplyWithRoot" 0 0))
        (Transformation|AttachComponentToComponent _returnvalue_3 _firespawnpointmid_2 "None" "KeepWorld" "KeepWorld" "KeepWorld" true)
        (Variables|Default|SetBaseFirerate 0.8))
      (:2
        (bind _returnvalue_4 (Game|SpawnActorfromClass "/Game/Blueprints/BulletsAndSummons/BP_PBullet_SwordTier3.BP_PBullet_SwordTier3_C" (Math|Transform|MakeTransform (.location _returnvalue) (.rotation _returnvalue) "1.000000,1.000000,1.000000") "AlwaysSpawn" "MultiplyWithRoot" 0 0))
        (Transformation|AttachComponentToComponent _returnvalue_4 _firespawnpointmid_2 "None" "KeepWorld" "KeepWorld" "KeepWorld" true)
        (Variables|Default|SetBaseFirerate 0.7)))
    (bind _newfirerate (CallFunction|FirerateCalculation (Variables|Default|GetBaseFirerate)))
    (Utilities|Time|SetTimerbyFunctionName 0 "FireCoolDown" _newfirerate)))

(fn ConstructionScript
  (|CallParentFunction))