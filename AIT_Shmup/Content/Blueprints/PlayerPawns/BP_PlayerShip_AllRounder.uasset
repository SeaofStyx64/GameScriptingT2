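; BP_PlayerShip_AllRounder is the all-rounder player ship pawn, defining how that ship fires its weapon.
; FireWeapon checks CanFireWeapon, plays a quiet laser sound at random pitch, and spawns a basic bullet, alternating between left and right spawn points via FlipFlop.
; It then blocks firing and starts the FireCoolDown timer by function name, with the delay derived from FirerateCalculation.
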(event EventBeginPlay
  (|CallParentFunction) ; This node is disabled and will not be called.\nDrag off pins to build functionality.
)

(event Collision|EventActorBeginOverlap
  (params (OtherActor :type Actor%20Object%20Reference)))

(event EventTick
  (params (DeltaSeconds :type Float%20%28single-precision%29))
  (|CallParentFunction DeltaSeconds) ; This node is disabled and will not be called.\nDrag off pins to build functionality.
)

(event EventFireWeapon
  (if (Variables|Default|GetCanFireWeapon)
    (Variables|Default|SetIsFiringWeapon true)
    (Audio|PlaySound2D "/Game/SoundFX/Laser1.Laser1" 0.2 (Math|Random|RandomFloatinRange 0.5 1.0) 0.0 0 0)
    (Utilities|FlowControl|FlipFlop
      (:A
        (Game|SpawnActorfromClass "/Game/Blueprints/BulletsAndSummons/BP_PBullet_Basic.BP_PBullet_Basic_C" (Transformation|GetWorldTransform (Variables|Default|GetFireSpawnPointLeft)) "AlwaysSpawn" "MultiplyWithRoot" 0 0))
      (:B
        (Game|SpawnActorfromClass "/Game/Blueprints/BulletsAndSummons/BP_PBullet_Basic.BP_PBullet_Basic_C" (Transformation|GetWorldTransform (Variables|Default|GetFireSpawnPointRight)) "AlwaysSpawn" "MultiplyWithRoot" 0 0)))
    (Variables|Default|SetCanFireWeapon false)
    (bind _newfirerate (CallFunction|FirerateCalculation 0.2))
    (Utilities|Time|SetTimerbyFunctionName 0 "FireCoolDown" _newfirerate)))

(fn ConstructionScript
  (|CallParentFunction))