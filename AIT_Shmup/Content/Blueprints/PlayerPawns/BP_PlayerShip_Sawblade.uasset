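; BP_PlayerShip_Sawblade is a player ship variant that fires sawblade projectiles.
; FireWeapon, gated by CanFireWeapon, plays a randomly pitched charge-up sound and spawns BP_PBullet_Sawblade at the middle fire point.
; Weapon tier 1 spawns an enlarged blade, while any other tier spawns one at default scale.
; After firing, it blocks further shots and starts a FireCoolDown timer timed by FirerateCalculation.
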(event EventFireWeapon
  (bind _firespawnpointmid (Variables|Default|GetFireSpawnPointMid))
  (bind _returnvalue (Transformation|GetWorldTransform _firespawnpointmid))
  (if (Variables|Default|GetCanFireWeapon)
    (Variables|Default|SetIsFiringWeapon true)
    (Audio|PlaySound2D "/Game/SoundFX/Chargeup.Chargeup" 1.0 (Math|Random|RandomFloatinRange 0.8 1.0) 0.0 0 0)
    (switch int (Variables|Default|GetWeaponTier)
      (:Default
        (Game|SpawnActorfromClass "/Game/Blueprints/BulletsAndSummons/BP_PBullet_Sawblade.BP_PBullet_Sawblade_C" (Math|Transform|MakeTransform (.location _returnvalue) (.rotation _returnvalue) "1.000000,1.000000,1.000000") "AlwaysSpawn" "MultiplyWithRoot" 0 0 :!label _label))
      (:0
        (goto _label))
      (:1
        (Game|SpawnActorfromClass "/Game/Blueprints/BulletsAndSummons/BP_PBullet_Sawblade.BP_PBullet_Sawblade_C" (Math|Transform|MakeTransform (.location _returnvalue) (.rotation _returnvalue) "2.500000,2.500000,2.500000") "AlwaysSpawn" "MultiplyWithRoot" 0 0)))
    (Variables|Default|SetCanFireWeapon false)
    (bind _newfirerate (CallFunction|FirerateCalculation 1.6))
    (Utilities|Time|SetTimerbyFunctionName 0 "FireCoolDown" _newfirerate)))

(fn ConstructionScript
  (|CallParentFunction))