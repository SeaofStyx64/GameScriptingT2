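; Player ship pawn for a shooter, steered along world axes with Enhanced Input and banked visually toward sideways input.
; Debug keys Q/E step through four weapons (alternating-barrel basic, triple shot, sawblade, beam), updating the HUD.
; Held fire is paced by per-weapon Delay nodes before each projectile spawn.
; Bullet or enemy overlaps cost health, flash an overlay and update the HUD; death spawns particles, disables input, then quits the game.
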(event OnComponentBeginOverlap(Box)
  (params (OverlappedComponent :type Primitive%20Component%20Object%20Reference) (OtherActor :type Actor%20Object%20Reference) (OtherComp :type Primitive%20Component%20Object%20Reference) (OtherBodyIndex :type Integer) (bFromSweep :type Boolean) (SweepResult :type Hit%20Result%20Structure%20%28by%20ref%29))
  ;[0.15 0.15 0.15 0.5] When Contacting Other Object
  (bind _asbp_bullet (Utilities|Casting|CastToBP_Bullet OtherActor)
    (:then
      (CallFunction|ApplyDamagetoPlayer (Variables|/Game/Blueprints/BP_Bullet.BP_Bullet_C|GetDamage _asbp_bullet)))
    (:CastFailed
      (bind _asbp_enemy_base (Utilities|Casting|CastToBP_Enemy_Base OtherActor))
      (Default|GetHitbyPlayer _asbp_enemy_base)
      (CallFunction|ApplyDamagetoPlayer (Variables|/Game/Blueprints/BP_Enemy_Base.BP_Enemy_Base_C|GetContactDamage _asbp_enemy_base)))))

(event Custom|ApplyDamageToPlayer
  (params (DamageTaken :type Float%20%28double-precision%29))
  ;[0.15 0.15 0.15 0.5] Applying Damage Taken When Hit
  (Variables|Default|SetHealth (- (Variables|Default|GetHealth) DamageTaken))
  (CallFunction|DamageOverlay)
  (Audio|PlaySound2D "/Game/SoundFX/PlayerHit.PlayerHit" 1.0 1.0 0.0 0 0)
  (bind _asbp_my_hud (Utilities|Casting|CastToBP_MyHUD (HUD|GetHUD (Game|GetPlayerController 0))))
  (Default|TakeDamage (Variables|/Game/Framework/BP_MyHUD.BP_MyHUD_C|GetUI%20Ref _asbp_my_hud) (/ (Variables|Default|GetHealth) (Variables|Default|GetMaxHealth)))
  (if (<= (Variables|Default|GetHealth) 0.0)
    (Audio|PlaySound2D "/Game/SoundFX/Explosion1.Explosion1" 1.0 (Math|Random|RandomFloatinRange 0.5 1.0) 0.0 0 0)
    (Rendering|SetVisibility (Variables|Default|GetShipModel) false false)
    (Game|SpawnActorfromClass "/Game/Particles/BP_PlayerDeathParticle.BP_PlayerDeathParticle_C" (Transformation|GetActorTransform) "AlwaysSpawn" "MultiplyWithRoot" 0 0)
    (Input|DisableInput (Game|GetPlayerController 0))
    (Utilities|FlowControl|Delay 1.5)
    (Actor|DestroyActor)
    (Game|QuitGame (Game|GetPlayerController 0) "Quit" false)))

(event Custom|DamageOverlay
  (Rendering|Material|SetOverlayMaterial (Variables|Default|GetShipModel) "/Game/Materials/M_DamageOverlay_Player.M_DamageOverlay_Player" :!class /Script/Engine.MeshComponent)
  (Utilities|FlowControl|Delay 0.2)
  (Rendering|Material|SetOverlayMaterial (Variables|Default|GetShipModel) 0 :!class /Script/Engine.MeshComponent))

(event Input|EnhancedActionEvents|EnhancedInputActionIA_Forward
  (params (ActionValue :type Boolean) (ElapsedSeconds :type Float%20%28double-precision%29) (TriggeredSeconds :type Float%20%28double-precision%29) (InputAction :type Input%20Action%20Object%20Reference :default "/Game/Data/IA_Forward.IA_Forward"))
  ;[0.15 0.15 0.15 0.5] Movement
  (Class|PawnMovementComponent|AddInputVector (Variables|Default|GetFloatingPawnMovement) "1.000000,0.000000,0.000000" false))

(event Input|EnhancedActionEvents|EnhancedInputActionIA_Right
  (params (ActionValue :type Boolean) (ElapsedSeconds :type Float%20%28double-precision%29) (TriggeredSeconds :type Float%20%28double-precision%29) (InputAction :type Input%20Action%20Object%20Reference :default "/Game/Data/IA_Right.IA_Right"))
  ;[0.15 0.15 0.15 0.5] Movement
  (Class|PawnMovementComponent|AddInputVector (Variables|Default|GetFloatingPawnMovement) "0.000000,1.000000,0.000000" false))

(event Input|EnhancedActionEvents|EnhancedInputActionIA_PrimaryShoot
  (params (ActionValue :type Boolean) (ElapsedSeconds :type Float%20%28double-precision%29) (TriggeredSeconds :type Float%20%28double-precision%29) (InputAction :type Input%20Action%20Object%20Reference :default "/Game/Data/IA_PrimaryShoot.IA_PrimaryShoot"))
  (:Triggered
    (switch int (Variables|Default|GetBulletType)
      (:0
        ;[0.15 0.15 0.15 0.5] Shoot (basic)
        (Utilities|FlowControl|Delay 0.05)
        (Audio|PlaySound2D "/Game/SoundFX/Laser1.Laser1" 0.2 (Math|Random|RandomFloatinRange 0.5 1.0) 0.0 0 0)
        (Utilities|FlowControl|FlipFlop
          (:A
            (Game|SpawnActorfromClass "/Game/Blueprints/BP_Bullet_Basic.BP_Bullet_Basic_C" (Transformation|GetWorldTransform (Variables|Default|GetFireSpawnPointLeft)) "AlwaysSpawn" "MultiplyWithRoot" 0 0))
          (:B
            (Game|SpawnActorfromClass "/Game/Blueprints/BP_Bullet_Basic.BP_Bullet_Basic_C" (Transformation|GetWorldTransform (Variables|Default|GetFireSpawnPointRight)) "AlwaysSpawn" "MultiplyWithRoot" 0 0))))
      (:1
        ;[0.15 0.15 0.15 0.5] Shoot (triple)
        (Utilities|FlowControl|Delay 0.2)
        (Audio|PlaySound2D "/Game/SoundFX/Laser2Mono.Laser2Mono" 0.2 (Math|Random|RandomFloatinRange 0.4 1.0) 0.0 0 0)
        (Game|SpawnActorfromClass "/Game/Blueprints/BP_Bullet_TripleShot.BP_Bullet_TripleShot_C" (Math|Transform|MakeTransform (Transformation|GetWorldLocation (Variables|Default|GetFireSpawnPointMid)) "0, 0, 0" "1.000000,1.000000,1.000000") "AlwaysSpawn" "MultiplyWithRoot" 0 0)
        (Game|SpawnActorfromClass "/Game/Blueprints/BP_Bullet_TripleShot.BP_Bullet_TripleShot_C" (Math|Transform|MakeTransform (Transformation|GetWorldLocation (Variables|Default|GetFireSpawnPointMid)) "0.000000,30.000000,0.000000" "1.000000,1.000000,1.000000") "AlwaysSpawn" "MultiplyWithRoot" 0 0)
        (Game|SpawnActorfromClass "/Game/Blueprints/BP_Bullet_TripleShot.BP_Bullet_TripleShot_C" (Math|Transform|MakeTransform (Transformation|GetWorldLocation (Variables|Default|GetFireSpawnPointMid)) "0.000000,-30.000000,0.000000" "1.000000,1.000000,1.000000") "AlwaysSpawn" "MultiplyWithRoot" 0 0))
      (:2
        ;[0.15 0.15 0.15 0.5] Sawblade
        (Utilities|FlowControl|Delay 1.0)
        (Audio|PlaySound2D "/Game/SoundFX/Chargeup.Chargeup" 1.0 (Math|Random|RandomFloatinRange 0.8 1.0) 0.0 0 0)
        (Game|SpawnActorfromClass "/Game/Blueprints/BP_Bullet_Sawblade.BP_Bullet_Sawblade_C" (Transformation|GetWorldTransform (Variables|Default|GetFireSpawnPointMid)) "AlwaysSpawn" "MultiplyWithRoot" 0 0))
      (:3
        ;[0.15 0.15 0.15 0.5] Beam
        (Utilities|FlowControl|Delay 0.0)
        (Audio|PlaySound2D "/Engine/EditorSounds/GamePreview/EjectFromPlayer.EjectFromPlayer" 1e+02 (Math|Random|RandomFloat) 0.0 0 0)
        (Game|SpawnActorfromClass "/Game/Blueprints/BP_Bullet_Beam.BP_Bullet_Beam_C" (Transformation|GetWorldTransform (Variables|Default|GetFireSpawnPointMid)) "AlwaysSpawn" "MultiplyWithRoot" 0 0)))))

(event Input|EnhancedActionEvents|EnhancedInputActionIA_Left
  (params (ActionValue :type Boolean) (ElapsedSeconds :type Float%20%28double-precision%29) (TriggeredSeconds :type Float%20%28double-precision%29) (InputAction :type Input%20Action%20Object%20Reference :default "/Game/Data/IA_Left.IA_Left"))
  ;[0.15 0.15 0.15 0.5] Movement
  (Class|PawnMovementComponent|AddInputVector (Variables|Default|GetFloatingPawnMovement) "0.000000,-1.000000,0.000000" false))

(event Input|EnhancedActionEvents|EnhancedInputActionIA_Backwards
  (params (ActionValue :type Boolean) (ElapsedSeconds :type Float%20%28double-precision%29) (TriggeredSeconds :type Float%20%28double-precision%29) (InputAction :type Input%20Action%20Object%20Reference :default "/Game/Data/IA_Backwards.IA_Backwards"))
  ;[0.15 0.15 0.15 0.5] Movement
  (Class|PawnMovementComponent|AddInputVector (Variables|Default|GetFloatingPawnMovement) "-1.000000,0.000000,0.000000" false))

(event EventBeginPlay
  ;[0.15 0.15 0.15 0.5] Add Mapping at Start
  (bind _asplayer_controller (Utilities|Casting|CastToPlayerController (Pawn|GetController)))
  (Input|AddMappingContext (PlayerController|LocalPlayerSubsystems|GetEnhancedInputLocalPlayerSubsystem _asplayer_controller) "/Game/Data/PlayerControlMapping.PlayerControlMapping" 0 "(bIgnoreAllPressedKeysUntilRelease=True,bForceImmediately=False,bNotifyUserSettings=False)"))

(event EventTick
  (params (DeltaSeconds :type Float%20%28single-precision%29))
  (bind _returnvalue (Input|EnhancedActionValues|GetIA_Right))
  (bind _returnvalue_2 (Input|EnhancedActionValues|GetIA_Left))
  (bind _returnvalue_3 (Math|Float|SelectFloat -1.0 0.0 _returnvalue))
  (bind _returnvalue_4 (Math|Float|SelectFloat 1.0 _returnvalue_3 _returnvalue_2))
  ;[0.15 0.15 0.15 0.5] Plane Roll
  (Variables|Default|SetTargetBankAngle _returnvalue_4)
  (Variables|Default|SetCurrentBankAngle (Math|Interpolation|FInterpTo (Variables|Default|GetCurrentBankAngle) _returnvalue_4 DeltaSeconds 8.0))
  (Transformation|SetRelativeRotation (Variables|Default|GetShipModel) (Math|Rotator|MakeRotator (* (Variables|Default|GetMaxBankAngle) (Variables|Default|GetCurrentBankAngle)) 0.0 1.8e+02) false false))

(event Input|KeyboardEvents|DebugKeyE
  (params (Key :type Key%20Structure :default "None") (ActionValue :type Input%20Action%20Value%20Structure))
  (bind _bullettype (Variables|Default|GetBulletType))
  ;[0.15 0.15 0.15 0.5] Bullet Variable Change and UI Cast
  (:Pressed
    (if (not (== _bullettype 3))
      (Math|Integer|IncrementInt _bullettype
        (:%20%20
          (bind _asbp_my_hud (Utilities|Casting|CastToBP_MyHUD (HUD|GetHUD (Game|GetPlayerController 0))))
          (Default|GunChangeUI (Variables|/Game/Framework/BP_MyHUD.BP_MyHUD_C|GetUI%20Ref _asbp_my_hud)))))))

(event Input|KeyboardEvents|DebugKeyQ
  (params (Key :type Key%20Structure :default "None") (ActionValue :type Input%20Action%20Value%20Structure))
  (bind _bullettype (Variables|Default|GetBulletType))
  ;[0.15 0.15 0.15 0.5] Bullet Variable Change and UI Cast
  (:Pressed
    (if (not (== _bullettype 0))
      (Math|Integer|DecrementInt _bullettype
        (:%20%20
          (bind _asbp_my_hud (Utilities|Casting|CastToBP_MyHUD (HUD|GetHUD (Game|GetPlayerController 0))))
          (Default|GunChangeUI (Variables|/Game/Framework/BP_MyHUD.BP_MyHUD_C|GetUI%20Ref _asbp_my_hud)))))))

(fn ConstructionScript)