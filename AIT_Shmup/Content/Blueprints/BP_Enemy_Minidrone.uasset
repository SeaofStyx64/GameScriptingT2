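; BP_Enemy_Minidrone is an enemy minidrone with a spinning sawblade.
; A Timeline started on BeginPlay drives the sawblade's relative yaw, and GetHitbyPlayer applies a fixed amount of damage through ApplyDamage.
; ShootBullet spawns an enemy bullet at BulletSpawnPoint, but the looping timer meant to fire it is disconnected, so nothing in this graph triggers shooting.
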(event Custom|ShootBullet
  (Game|SpawnActorfromClass "/Game/Blueprints/BP_Bullet_Enemy.BP_Bullet_Enemy_C" (Transformation|GetWorldTransform (Variables|Default|GetBulletSpawnPoint)) "Undefined" "MultiplyWithRoot" 0 0))

(event EventBeginPlay
  (bind _sawspinnew (Timeline|Timeline Play)
    (:Update
      (Transformation|SetRelativeRotation (Variables|Default|GetMinidroneSawblade) (Math|Rotator|MakeRotator 0.0 0.0 _sawspinnew) false false))))

(event EventGetHitbyPlayer
  (CallFunction|ApplyDamage 1e+02))

(fn ConstructionScript)