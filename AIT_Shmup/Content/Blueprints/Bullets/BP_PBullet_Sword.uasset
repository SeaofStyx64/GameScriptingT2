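; BP_PBullet_Sword is a bullet Blueprint that acts as a swinging sword blade instead of a flying projectile.
; On BeginPlay it runs the parent logic, then deactivates ProjectileMovement.
; A timeline drives the Blade component's relative yaw through the swing and destroys the actor when it finishes.
; It defines no active overlap or hit logic of its own.
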(event EventBeginPlay
  (|CallParentFunction)
  (Components|Activation|SetActive (Variables|Default|GetProjectileMovement) false false)
  (bind _bladeswing (Timeline|Timeline Play)
    (:Update
      (Transformation|SetRelativeRotation (Variables|Default|GetBlade) (Math|Rotator|MakeRotator 0.0 0.0 _bladeswing) false false))
    (:Finished
      (Actor|DestroyActor))))

(event Collision|EventActorBeginOverlap
  (params (OtherActor :type Actor%20Object%20Reference)))

(event EventTick
  (params (DeltaSeconds :type Float%20%28single-precision%29))
  (|CallParentFunction DeltaSeconds) ; This node is disabled and will not be called.\nDrag off pins to build functionality.
)

(fn ConstructionScript
  (|CallParentFunction))