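; Level 2 sword player bullet that acts as a double-blade swing attack rather than a moving projectile.
; On BeginPlay it deactivates its ProjectileMovement, then starts two timelines that animate the relative yaw of Blade1 and Blade2.
; The actor destroys itself as soon as either swing timeline finishes.
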(event EventBeginPlay
  (|CallParentFunction)
  (Components|Activation|SetActive (Variables|Default|GetProjectileMovement) false false)
  (Utilities|FlowControl|Sequence
    (:then_0
      (bind _bladeswing (Timeline|Blade1Swing Play)
        (:Update
          (Transformation|SetRelativeRotation (Variables|Default|GetBlade1) (Math|Rotator|MakeRotator 0.0 0.0 _bladeswing) false false))
        (:Finished
          (Actor|DestroyActor :!label _label))))
    (:then_1
      (bind _bladeswing2 (Timeline|Blade2Swing Play)
        (:Update
          (Transformation|SetRelativeRotation (Variables|Default|GetBlade2) (Math|Rotator|MakeRotator 0.0 0.0 _bladeswing2) false false))
        (:Finished
          (goto _label))))))

(event Collision|EventActorBeginOverlap
  (params (OtherActor :type Actor%20Object%20Reference)))

(event EventTick
  (params (DeltaSeconds :type Float%20%28single-precision%29))
  (|CallParentFunction DeltaSeconds) ; This node is disabled and will not be called.\nDrag off pins to build functionality.
)

(fn ConstructionScript
  (|CallParentFunction))