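; Shotgunner enemy that travels on projectile movement for a few seconds, then stops to fire three-bullet spreads at the player.
; After a random delay it deactivates movement, shoots, and starts a looping shot timer with an interval randomized once.
; A Timeline eases its yaw toward the player, and each briefly delayed volley spawns bullets 45 degrees apart with multiplied damage.
; GetHitbyPlayer applies fixed damage through ApplyDamage.
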(event Custom|ShootBullet
  (bind _bulletspawnpoint (Variables|Default|GetBulletSpawnPoint))
  (bind _returnvalue (Transformation|GetWorldTransform _bulletspawnpoint))
  (Variables|Default|SetShootAngle "0.000000,-45.000000,0.000000")
  (Utilities|FlowControl|Delay 0.3)
  (for _index (range 0 2)
    (bind _returnvalue_2 (Game|SpawnActorfromClass "/Game/Blueprints/BulletsAndSummons/BP_EBullet_Basic.BP_EBullet_Basic_C" (Math|Transform|MakeTransform (.location _returnvalue) (Math|Rotator|MakeRotator (.roll (.rotation _returnvalue)) (.pitch (.rotation _returnvalue)) (+ (.yaw (.rotation _returnvalue)) (.yaw (Variables|Default|GetShootAngle)))) "1.000000,1.000000,1.000000") "AlwaysSpawn" "MultiplyWithRoot" 0 0))
    (Variables|/Game/Blueprints/BulletsAndSummons/BP_BaseEnemyBullet.BP_BaseEnemyBullet_C|SetDamage _returnvalue_2 (* (Variables|/Game/Blueprints/BulletsAndSummons/BP_BaseEnemyBullet.BP_BaseEnemyBullet_C|GetDamage _returnvalue_2) (Variables|Default|GetProjectileDamageMult)))
    (Variables|Default|SetShootAngle (Math|Rotator|MakeRotator 0.0 0.0 (+ (.yaw (Variables|Default|GetShootAngle)) 45.0)))))

(event EventBeginPlay
  (Utilities|FlowControl|Delay (Math|Random|RandomFloatinRange 4.0 5.0))
  (Components|Activation|Deactivate (Variables|Default|GetProjectileMovement))
  (CallFunction|ShootBullet)
  (bind _returnvalue (Utilities|Time|SetTimerbyEvent (delegate Custom|ShootBullet) (Math|Random|RandomFloatinRange 1.0 3.0) true true))
  (Variables|Default|SetShootTimer _returnvalue)
  (Timeline|Timeline PlayFromStart
    (:Update
      (Transformation|SetActorRotation (Math|Rotator|MakeRotator 0.0 0.0 (.yaw (Math|Rotator|Lerp(Rotator) (Math|Rotator|MakeRotator 0.0 0.0 (.yaw (Transformation|GetActorRotation))) (Math|Rotator|MakeRotator 0.0 0.0 (.yaw (Math|Rotator|FindLookatRotation (Transformation|GetWorldLocation (Variables|Default|GetDefaultSceneRoot)) (Transformation|GetActorLocation (Game|Player|GetPlayerPawn 0))))) 0.08 true)))))))

(event EventGetHitbyPlayer
  (CallFunction|ApplyDamage 1e+02))

(fn ConstructionScript)