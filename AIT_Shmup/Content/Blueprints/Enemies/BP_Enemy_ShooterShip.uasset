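; Enemy shooter ship that flies in on projectile movement, stops after a random few seconds, then fires at the player.
; A looping timer, with its interval randomized once, spawns BP_EBullet_Basic at the spawn point after a short delay, scaling damage by ProjectileDamageMult.
; Timeline updates serve as a tick to smoothly lerp the ship's yaw toward the player.
; A player hit applies fixed damage to the ship.
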(event Custom|ShootBullet
  (Utilities|FlowControl|Delay 0.3)
  (bind _returnvalue (Game|SpawnActorfromClass "/Game/Blueprints/BulletsAndSummons/BP_EBullet_Basic.BP_EBullet_Basic_C" (Transformation|GetWorldTransform (Variables|Default|GetBulletSpawnPoint)) "AlwaysSpawn" "MultiplyWithRoot" 0 0))
  (Variables|/Game/Blueprints/BulletsAndSummons/BP_BaseEnemyBullet.BP_BaseEnemyBullet_C|SetDamage _returnvalue (* (Variables|/Game/Blueprints/BulletsAndSummons/BP_BaseEnemyBullet.BP_BaseEnemyBullet_C|GetDamage _returnvalue) (Variables|Default|GetProjectileDamageMult))))

(event EventBeginPlay
  (Utilities|FlowControl|Delay (Math|Random|RandomFloatinRange 4.0 5.0))
  (Components|Activation|Deactivate (Variables|Default|GetProjectileMovement))
  (CallFunction|ShootBullet)
  (bind _returnvalue (Utilities|Time|SetTimerbyEvent (delegate Custom|ShootBullet) (Math|Random|RandomFloatinRange 1.0 3.0) true true))
  (Variables|Default|SetShootTimer _returnvalue)
  (Timeline|Timeline PlayFromStart
    (:Update
      (Transformation|SetActorRotation (Math|Rotator|MakeRotator 0.0 0.0 (.yaw (Math|Rotator|Lerp(Rotator) (Math|Rotator|MakeRotator 0.0 0.0 (.yaw (Transformation|GetActorRotation))) (Math|Rotator|MakeRotator 0.0 0.0 (.yaw (Math|Rotator|FindLookatRotation (Transformation|GetWorldLocation (Variables|Default|GetDefaultSceneRoot)) (Transformation|GetActorLocation (Game|Player|GetPlayerPawn 0))))) 0.08 true)))))))

(event EventGetHitbyPlayer
  (CallFunction|ApplyDamage 1e+02))

(fn ConstructionScript)