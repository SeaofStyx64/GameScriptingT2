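; Bomb drone enemy that flies to a random spot, counts down, then explodes.
; On BeginPlay it takes its target from BP_RandomEnemyAimFor, faces it and starts a timeline that spins the Drone component.
; Tick drives FloatingPawnMovement until arrival, when movement stops and a Countdown timeline shifts the material from green to red.
; When the countdown ends, it spawns BP_BulletExplosion with its projectile damage multiplier and destroys itself.
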(event Custom|FoundSpot
  (Variables|Default|SetFoundLocation true)
  (Components|Activation|Deactivate (Variables|Default|GetFloatingPawnMovement))
  (bind _timevalue (Timeline|Countdown Play)
    (:Update
      (Rendering|Material|SetVectorParameterValueonMaterials (Variables|Default|GetDrone) "Colour" (Math|Vector|Lerp(Vector) "0.000000,1.000000,0.000000" "0.500000,0.000000,0.000000" _timevalue)))
    (:Finished
      (bind _returnvalue (Game|SpawnActorfromClass "/Game/Blueprints/BulletsAndSummons/BP_BulletExplosion.BP_BulletExplosion_C" (Math|Transform|MakeTransform (.location (Transformation|GetActorTransform)) "0, 0, 0" "1.000000,1.000000,1.000000") "AlwaysSpawn" "MultiplyWithRoot" 0 0))
      (Variables|/Game/Blueprints/BulletsAndSummons/BP_BulletExplosion.BP_BulletExplosion_C|SetDamageMult _returnvalue (Variables|Default|GetProjectileDamageMult))
      (Actor|DestroyActor))))

(event Custom|MoveTowardsTarget
  (Class|PawnMovementComponent|AddInputVector (Variables|Default|GetFloatingPawnMovement) (Math|Vector|GetUnitDirection(Vector) (Transformation|GetActorLocation) (Variables|Default|GetTargetLocation)) false)
  (if (Utilities|Operators|EqualEqual (Variables|Default|GetTargetLocation) (Transformation|GetActorLocation) 1e+01)
    (CallFunction|FoundSpot)))

(event EventBeginPlay
  (|CallParentFunction)
  (Utilities|FlowControl|Sequence
    (:then_0
      (bind _spin (Timeline|Spiinnnn Play)
        (:Update
          (Transformation|SetRelativeRotation (Variables|Default|GetDrone) (Math|Rotator|MakeRotator 0.0 0.0 _spin) false false))))
    (:then_1
      (bind _returnvalue (Actor|GetActorOfClass "/Game/Blueprints/BP_RandomEnemyAimFor.BP_RandomEnemyAimFor_C"))
      (bind _output_get (Variables|Default|SetTargetLocation (Variables|/Game/Blueprints/BP_RandomEnemyAimFor.BP_RandomEnemyAimFor_C|GetRandomSpot _returnvalue)))
      (Transformation|SetActorRotation (Math|Rotator|FindLookatRotation (Transformation|GetActorLocation) _output_get)))))

(event EventTick
  (params (DeltaSeconds :type Float%20%28single-precision%29))
  (if (not (Variables|Default|GetFoundLocation))
    (CallFunction|MoveTowardsTarget)))

(fn ConstructionScript
  (|CallParentFunction))