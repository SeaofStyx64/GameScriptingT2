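; Segmented snake drone enemy for a shoot-'em-up that flies in a straight line toward where the player was at BeginPlay.
; Tick feeds that fixed direction to FloatingPawnMovement, and a timer destroys it after Lifespan.
; A Timeline fakes slithering by offsetting segments sideways, mostly in alternating directions, and yawing the tail.
; EnemyDeathSequence disables movement and collision, adds score via the HUD, then staggers death particles from head to tail before destroying itself.
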(event Custom|DestroySelf
  (Actor|DestroyActor))

(event EventBeginPlay
  (bind _body5 (Variables|Default|GetBody5))
  (bind _tail (Variables|Default|GetTail))
  (bind _body1 (Variables|Default|GetBody1))
  (bind _head (Variables|Default|GetHead))
  (bind _body3 (Variables|Default|GetBody3))
  (bind _body2 (Variables|Default|GetBody2))
  (bind _body4 (Variables|Default|GetBody4))
  (bind _returnvalue (Transformation|GetRelativeTransform _body2))
  (bind _returnvalue_2 (Transformation|GetRelativeTransform _body3))
  (bind _returnvalue_3 (Transformation|GetRelativeTransform _tail))
  (bind _returnvalue_4 (Transformation|GetRelativeTransform _body5))
  (bind _returnvalue_5 (Transformation|GetRelativeTransform _body1))
  (bind _returnvalue_6 (Transformation|GetRelativeTransform _body4))
  (bind _returnvalue_7 (Transformation|GetRelativeTransform _head))
  (|CallParentFunction)
  (Variables|Default|SetMovementDirection (Math|Vector|GetUnitDirection(Vector) (Transformation|GetActorLocation) (Transformation|GetActorLocation (Game|Player|GetPlayerPawn 0))))
  (Utilities|Time|SetTimerbyEvent (delegate Custom|DestroySelf) (Variables|Default|GetLifespan))
  (Transformation|SetActorRotation (Math|Rotator|FindLookatRotation (Transformation|GetActorLocation) (Transformation|GetActorLocation (Game|Player|GetPlayerPawn 0))))
  (bind _slither (Timeline|Timeline Play)
    (:Update
      (Variables|Default|SetSlitherValue _slither)
      (Transformation|SetRelativeLocation _head (Math|Vector|MakeVector (.x (.location _returnvalue_7)) (* (Variables|Default|GetSlitherValue) -1.0) (.z (.location _returnvalue_7))) false false)
      (Transformation|SetRelativeLocation _body1 (Math|Vector|MakeVector (.x (.location _returnvalue_5)) (Variables|Default|GetSlitherValue) (.z (.location _returnvalue_5))) false false)
      (Transformation|SetRelativeLocation _body2 (Math|Vector|MakeVector (.x (.location _returnvalue)) (* (Variables|Default|GetSlitherValue) -1.0) (.z (.location _returnvalue))) false false)
      (Transformation|SetRelativeLocation _body3 (Math|Vector|MakeVector (.x (.location _returnvalue_2)) (Variables|Default|GetSlitherValue) (.z (.location _returnvalue_2))) false false)
      (Transformation|SetRelativeLocation _body4 (Math|Vector|MakeVector (.x (.location _returnvalue_6)) (* (Variables|Default|GetSlitherValue) -1.0) (.z (.location _returnvalue_6))) false false)
      (Transformation|SetRelativeLocation _body5 (Math|Vector|MakeVector (.x (.location _returnvalue_4)) (Variables|Default|GetSlitherValue) (.z (.location _returnvalue_4))) false false)
      (Transformation|SetRelativeLocation _tail (Math|Vector|MakeVector (.x (.location _returnvalue_3)) (Variables|Default|GetSlitherValue) (.z (.location _returnvalue_3))) false false)
      (Transformation|SetRelativeRotation _tail (Math|Rotator|MakeRotator 0.0 0.0 (+ (Variables|Default|GetSlitherValue) -9e+01)) false false))))

(event EventEnemyDeathSequence
  (Components|Activation|SetActive (Variables|Default|GetFloatingPawnMovement) false false)
  (Collision|SetActorEnableCollision false)
  (Audio|PlaySound2D "/Game/SoundFX/Explosion1.Explosion1" 0.5 (Math|Random|RandomFloatinRange 0.5 1.0) 0.0 0 0)
  (bind _asbp_shmup_hud (Utilities|Casting|CastToBP_ShmupHUD (HUD|GetHUD (Game|GetPlayerController 0))))
  (Default|IncreaseScore (Variables|/Game/Framework/BP_ShmupHUD.BP_ShmupHUD_C|GetUI%20Ref _asbp_shmup_hud) (Variables|Default|GetLootScore))
  (Game|SpawnActorfromClass "/Game/Particles/BP_EnemyDeathParticle.BP_EnemyDeathParticle_C" (Math|Transform|MakeTransform (Transformation|GetWorldLocation (Variables|Default|GetHead)) "0, 0, 0" "1.000000,1.000000,1.000000") "AlwaysSpawn" "MultiplyWithRoot" 0 0)
  (Utilities|FlowControl|Delay 0.1)
  (Game|SpawnActorfromClass "/Game/Particles/BP_EnemyDeathParticle.BP_EnemyDeathParticle_C" (Math|Transform|MakeTransform (Transformation|GetWorldLocation (Variables|Default|GetBody1)) "0, 0, 0" "1.000000,1.000000,1.000000") "AlwaysSpawn" "MultiplyWithRoot" 0 0)
  (Utilities|FlowControl|Delay 0.1)
  (Game|SpawnActorfromClass "/Game/Particles/BP_EnemyDeathParticle.BP_EnemyDeathParticle_C" (Math|Transform|MakeTransform (Transformation|GetWorldLocation (Variables|Default|GetBody2)) "0, 0, 0" "1.000000,1.000000,1.000000") "AlwaysSpawn" "MultiplyWithRoot" 0 0)
  (Utilities|FlowControl|Delay 0.1)
  (Game|SpawnActorfromClass "/Game/Particles/BP_EnemyDeathParticle.BP_EnemyDeathParticle_C" (Math|Transform|MakeTransform (Transformation|GetWorldLocation (Variables|Default|GetBody3)) "0, 0, 0" "1.000000,1.000000,1.000000") "AlwaysSpawn" "MultiplyWithRoot" 0 0)
  (Utilities|FlowControl|Delay 0.1)
  (Game|SpawnActorfromClass "/Game/Particles/BP_EnemyDeathParticle.BP_EnemyDeathParticle_C" (Math|Transform|MakeTransform (Transformation|GetWorldLocation (Variables|Default|GetBody4)) "0, 0, 0" "1.000000,1.000000,1.000000") "AlwaysSpawn" "MultiplyWithRoot" 0 0)
  (Utilities|FlowControl|Delay 0.1)
  (Game|SpawnActorfromClass "/Game/Particles/BP_EnemyDeathParticle.BP_EnemyDeathParticle_C" (Math|Transform|MakeTransform (Transformation|GetWorldLocation (Variables|Default|GetBody5)) "0, 0, 0" "1.000000,1.000000,1.000000") "AlwaysSpawn" "MultiplyWithRoot" 0 0)
  (Utilities|FlowControl|Delay 0.1)
  (Game|SpawnActorfromClass "/Game/Particles/BP_EnemyDeathParticle.BP_EnemyDeathParticle_C" (Math|Transform|MakeTransform (Transformation|GetWorldLocation (Variables|Default|GetTail)) "0, 0, 0" "1.000000,1.000000,1.000000") "AlwaysSpawn" "MultiplyWithRoot" 0 0)
  (Actor|DestroyActor))

(event EventTick
  (params (DeltaSeconds :type Float%20%28single-precision%29))
  (Class|PawnMovementComponent|AddInputVector (Variables|Default|GetFloatingPawnMovement) (Variables|Default|GetMovementDirection) false))

(fn ConstructionScript
  (|CallParentFunction))