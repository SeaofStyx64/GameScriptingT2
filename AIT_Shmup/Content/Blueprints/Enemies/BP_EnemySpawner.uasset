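; Enemy spawner that runs timed waves, advancing every 30 seconds and continuously spawning enemies at random intervals.
; Each spawn picks random points on start and end splines, faces the end point, and draws a random class from the current wave's pool.
; That wave's data scales health, damage and loot score and sets the next spawn interval.
; Waves 9, 19, 29 and 39 are flagged as boss waves, but only 9 spawns a boss, the SnakeDrone.
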(event Custom|SpawnEnemy
  (bind (_startlocation _endlocation) (CallFunction|GetStart&EndLocation))
  (Variables|Default|SetSpawnTrans (Math|Transform|MakeTransform _startlocation (Math|Rotator|FindLookatRotation _startlocation _endlocation) "1.000000,1.000000,1.000000"))
  (bind _array_element (Utilities|Array|ForEachLoopwithBreak (Variables|Default|GetWaveInfo) :!label _label)
    (:LoopBody
      (if (== (.WaveID (Utilities|Struct|BreakEnemySpawnWaves _array_element)) (Variables|Default|GetCurrentWave))
        (goto _label Break)))
    (:Completed
      (bind _returnvalue (Game|SpawnActorfromClass (.OutItem (Utilities|Array|Random (.EnemyPool (Utilities|Struct|BreakEnemySpawnWaves _array_element)))) (Variables|Default|GetSpawnTrans) "AlwaysSpawn" "MultiplyWithRoot" 0 0))
      (Variables|/Game/Blueprints/Enemies/BP_Enemy_Base.BP_Enemy_Base_C|SetMaxHealth _returnvalue (* (Variables|/Game/Blueprints/Enemies/BP_Enemy_Base.BP_Enemy_Base_C|GetMaxHealth _returnvalue) (.HealthMult (Utilities|Struct|BreakEnemySpawnWaves _array_element))))
      (Variables|/Game/Blueprints/Enemies/BP_Enemy_Base.BP_Enemy_Base_C|SetHealth _returnvalue (* (Variables|/Game/Blueprints/Enemies/BP_Enemy_Base.BP_Enemy_Base_C|GetHealth _returnvalue) (.HealthMult (Utilities|Struct|BreakEnemySpawnWaves _array_element))))
      (Variables|/Game/Blueprints/Enemies/BP_Enemy_Base.BP_Enemy_Base_C|SetContactDamage _returnvalue (* (Variables|/Game/Blueprints/Enemies/BP_Enemy_Base.BP_Enemy_Base_C|GetContactDamage _returnvalue) (.DamageMult (Utilities|Struct|BreakEnemySpawnWaves _array_element))))
      (Variables|/Game/Blueprints/Enemies/BP_Enemy_Base.BP_Enemy_Base_C|SetProjectileDamageMult _returnvalue (.DamageMult (Utilities|Struct|BreakEnemySpawnWaves _array_element)))
      (Variables|/Game/Blueprints/Enemies/BP_Enemy_Base.BP_Enemy_Base_C|SetLootScore _returnvalue (* (Variables|/Game/Blueprints/Enemies/BP_Enemy_Base.BP_Enemy_Base_C|GetLootScore _returnvalue) (.ScoreMult (Utilities|Struct|BreakEnemySpawnWaves _array_element))))
      (Variables|Default|SetSpawnMin (.SpawnFrequencyMin (Utilities|Struct|BreakEnemySpawnWaves _array_element)))
      (Variables|Default|SetSpawnMax (.SpawnFrequencyMax (Utilities|Struct|BreakEnemySpawnWaves _array_element)))
      (CallFunction|QueueSpawn))))

(event Custom|QueueSpawn
  (Utilities|Time|SetTimerbyEvent (delegate Custom|SpawnEnemy) (Math|Random|RandomFloatinRangefromStream (Variables|Default|GetRandomStream) (Variables|Default|GetSpawnMin) (Variables|Default|GetSpawnMax)) false true))

(event Custom|SetNewWave
  (bind _output_get (Variables|Default|SetCurrentWave (+ (Variables|Default|GetCurrentWave) 1)))
  (Development|PrintString "Next Wave")
  (if (== _output_get (Class|KismetMathLibrary|OrIntInt 9 19 29 39))
    (Development|PrintString "BossWave")
    (if (== (Variables|Default|GetCurrentWave) 9)
      (CallFunction|TheGeneral)
      (elif (not (== (Variables|Default|GetCurrentWave) 19))
        (if (not (== (Variables|Default|GetCurrentWave) 19))
          (if (== (Variables|Default|GetCurrentWave) 19)
            _))))))

(event Custom|The%20General
  (Game|SpawnActorfromClass "/Game/Blueprints/Enemies/BP_Enemy_SnakeDrone.BP_Enemy_SnakeDrone_C" (Transformation|GetRelativeTransform (Variables|Default|GetBossSpawnLocation)) "AlwaysSpawn" "MultiplyWithRoot" 0 0))

(event EventBeginPlay
  (Math|Random|SetRandomStreamSeed (Variables|Default|GetRandomStream) 0)
  (CallFunction|QueueSpawn)
  (Utilities|Time|SetTimerbyEvent (delegate Custom|SetNewWave) 3e+01 true))

(fn ConstructionScript)

(fn GetStart&EndLocation
  (bind _randomstream (Variables|Default|GetRandomStream))
  (bind _returnvalue (Math|Random|RandomFloatfromStream _randomstream))
  (return (Spline|GetLocationatTime (Variables|Default|GetStartLocation) _returnvalue "World" false) (Spline|GetLocationatTime (Variables|Default|GetEndLocation) _returnvalue "World" false)))