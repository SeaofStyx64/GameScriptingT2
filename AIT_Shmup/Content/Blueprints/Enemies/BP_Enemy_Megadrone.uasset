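; BP_Enemy_Megadrone is an enemy drone with a spinning sawblade that destroys itself when its lifespan timer expires.
; BeginPlay starts that timer and plays a timeline that drives the sawblade's yaw rotation.
; Player hits apply fixed damage.
; ShootBullet spawns a basic enemy bullet at the spawn point, but the looping timer meant to trigger it is disconnected and never runs.
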(event Custom|ShootBullet
  (Game|SpawnActorfromClass "/Game/Blueprints/BulletsAndSummons/BP_EBullet_Basic.BP_EBullet_Basic_C" (Transformation|GetWorldTransform (Variables|Default|GetBulletSpawnPoint)) "Undefined" "MultiplyWithRoot" 0 0))

(event Custom|DestroySelf
  (Actor|DestroyActor))

(event Custom|GetHitByPlayer_1
  (CallFunction|ApplyDamage 1e+02))

(event EventBeginPlay
  (Utilities|Time|SetTimerbyEvent (delegate Custom|DestroySelf) (Variables|Default|GetLifespan))
  (bind _sawspinnew (Timeline|Timeline Play)
    (:Update
      (Transformation|SetRelativeRotation (Variables|Default|GetMinidroneSawblade) (Math|Rotator|MakeRotator 0.0 0.0 _sawspinnew) false false))))

(fn ConstructionScript)