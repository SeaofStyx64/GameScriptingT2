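; The General is a boss enemy that pursues the player while cycling through random attacks, starting on OnEnter.
; The ChaseDuration timeline smoothly yaws it toward the player and feeds movement input on each update.
; After a short delay, ChooseNewAttack draws from AttackPool: a temporary speed-boosted chase, a timed burst of double-damage bullets, or a random batch of homing missiles.
; Each attack calls ChooseNewAttack when finished, forming an endless loop.
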(event Custom|ChasePlayer
  (bind _floatingpawnmovement (Variables|Default|GetFloatingPawnMovement))
  ;[0.15 0.15 0.15 0.5] Chase Player
  (Variables|/Script/Engine.FloatingPawnMovement|SetMaxSpeed _floatingpawnmovement 8e+02)
  (Utilities|FlowControl|Delay 5.0)
  (Variables|/Script/Engine.FloatingPawnMovement|SetMaxSpeed _floatingpawnmovement 4e+02)
  (CallFunction|ChooseNewAttack))

(event Custom|ChooseNewAttack
  ;[0.15 0.15 0.15 0.5] Choose a random attack from a pool
  (Utilities|FlowControl|Delay 2.0)
  (switch name (.OutItem (Utilities|Array|Random (Variables|Default|GetAttackPool)))
    (:Default
      (CallFunction|ChasePlayer :!label _label))
    (:ChasePlayer
      (goto _label))
    (:FireBullets
      (CallFunction|FireBullets))
    (:SummonMissiles
      (CallFunction|SummonMissiles))))

(event Custom|FireBullets
  (bind _returnvalue (Transformation|GetActorTransform))
  ;[0.15 0.15 0.15 0.5] Fire Bullets
  (Variables|Default|SetBulletCount (Math|Random|RandomIntegerinRange 4 12))
  (bind _returnvalue_2 (Game|SpawnActorfromClass "/Game/Blueprints/BulletsAndSummons/BP_EBullet_Basic.BP_EBullet_Basic_C" (Math|Transform|MakeTransform (.location _returnvalue) (.rotation _returnvalue) "1.000000,1.000000,1.000000") "AlwaysSpawn" "MultiplyWithRoot" 0 0 :!label _label))
  (Variables|/Game/Blueprints/BulletsAndSummons/BP_BaseEnemyBullet.BP_BaseEnemyBullet_C|SetDamage _returnvalue_2 (* (Variables|/Game/Blueprints/BulletsAndSummons/BP_BaseEnemyBullet.BP_BaseEnemyBullet_C|GetDamage _returnvalue_2) 2.0))
  (if (<= (Variables|Default|GetBulletCount) 0)
    (CallFunction|ChooseNewAttack)
    (else
      (Variables|Default|SetBulletCount (- (Variables|Default|GetBulletCount) 1))
      (Utilities|FlowControl|Delay 0.2)
      (goto _label))))

(event Custom|SummonMissiles
  (bind _returnvalue (Transformation|GetActorLocation))
  (bind _returnvalue_2 (Class|KismetMathLibrary|RandomUnitVectorinConeinRadians _returnvalue 2e+02))
  ;[0.15 0.15 0.15 0.5] Summon Missiles
  (for _index (range 0 (Math|Random|RandomIntegerinRange 1 4))
    (Game|SpawnActorfromClass "/Game/Blueprints/Enemies/BP_Enemy_HomingMissile.BP_Enemy_HomingMissile_C" (Math|Transform|MakeTransform (Math|Vector|MakeVector (.x _returnvalue_2) (.y _returnvalue_2) 0.0) "0, 0, 0" "1.000000,1.000000,1.000000") "AlwaysSpawn" "MultiplyWithRoot" 0 0))
  (CallFunction|ChooseNewAttack))

(event EventOnEnter
  ;[0.15 0.15 0.15 0.5] Constant Rotate to face player
  (CallFunction|ChooseNewAttack)
  (Timeline|ChaseDuration PlayFromStart
    (:Update
      (Transformation|SetActorRotation (Math|Rotator|MakeRotator 0.0 0.0 (.yaw (Math|Rotator|Lerp(Rotator) (Math|Rotator|MakeRotator 0.0 0.0 (.yaw (Transformation|GetActorRotation))) (Math|Rotator|MakeRotator 0.0 0.0 (.yaw (Math|Rotator|FindLookatRotation (Transformation|GetActorLocation) (Transformation|GetActorLocation (Game|Player|GetPlayerPawn 0))))) 0.15 true))) true)
      (Class|PawnMovementComponent|AddInputVector (Variables|Default|GetFloatingPawnMovement) (Math|Vector|GetUnitDirection(Vector) (Transformation|GetActorLocation) (Transformation|GetActorLocation (Game|Player|GetPlayerPawn 0))) false))))

(fn ConstructionScript
  (|CallParentFunction))