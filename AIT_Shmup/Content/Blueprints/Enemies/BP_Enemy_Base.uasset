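; Base enemy actor for a shmup, handling red outline, damage intake, health bar and death.
; Capsule overlaps with player bullets or the player ship feed ApplyDamage, which doubles damage only when crit chance exactly equals a random float.
; Each hit updates the widget health bar, spawns a jittered number showing base damage, and briefly flashes mesh overlay materials.
; At zero health it spawns particles, plays an explosion, adds score and destroys itself next tick.
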(event OnComponentBeginOverlap(CapsuleHitbox)
  (params (OverlappedComponent :type Primitive%20Component%20Object%20Reference) (OtherActor :type Actor%20Object%20Reference) (OtherComp :type Primitive%20Component%20Object%20Reference) (OtherBodyIndex :type Integer) (bFromSweep :type Boolean) (SweepResult :type Hit%20Result%20Structure%20%28by%20ref%29))
  ;[0.15 0.15 0.15 0.5] Taking Damage + Contacting Bullets
  (bind _asbp_base_player_bullet (Utilities|Casting|CastToBP_BasePlayerBullet OtherActor)
    (:then
      (CallFunction|ApplyDamage (Variables|/Game/Blueprints/BulletsAndSummons/BP_BasePlayerBullet.BP_BasePlayerBullet_C|GetDamage _asbp_base_player_bullet)))
    (:CastFailed
      (bind _asbp_player_ship (Utilities|Casting|CastToBP_PlayerShip OtherActor))
      (CallFunction|ApplyDamage (Variables|/Game/Blueprints/BP_PlayerShip.BP_PlayerShip_C|GetContactDamage _asbp_player_ship)))))

(event Custom|Apply%20Damage
  (params (Damage :type Float%20%28double-precision%29))
  (bind _returnvalue (Transformation|GetActorLocation))
  (bind _returnvalue_2 (Math|Random|RandomFloatinRange -1e+02 1e+02))
  ;[0.15 0.15 0.15 0.5] Taking Damage + Contacting Bullets
  (bind _asbp_player_ship (Utilities|Casting|CastToBP_PlayerShip (Game|Player|GetPlayerPawn 0)))
  (if (== (Variables|/Game/Blueprints/BP_PlayerShip.BP_PlayerShip_C|GetUpgradeCritChance _asbp_player_ship) (Math|Random|RandomFloatinRange 0.0 1e+02))
    (Variables|Default|SetHealth (- (Variables|Default|GetHealth) (* Damage 2.0)))
    (Audio|PlaySound2D "/Engine/EditorSounds/GamePreview/PossessPlayer.PossessPlayer" 1.0 1.0 0.0 0 0)
    (else
      (Variables|Default|SetHealth (- (Variables|Default|GetHealth) Damage))))
  (bind _aswbp_enemy_health_bar (Utilities|Casting|CastToWBP_EnemyHealthBar (UserInterface|GetUserWidgetObject (Variables|Default|GetHealthbar))))
  (Default|SetHealth _aswbp_enemy_health_bar (/ (Variables|Default|GetHealth) (Variables|Default|GetMaxHealth)))
  (bind _returnvalue_3 (Game|SpawnActorfromClass "/Game/Blueprints/Indicators/BP_Indicator_Damage.BP_Indicator_Damage_C" (Math|Transform|MakeTransform (Math|Vector|MakeVector (+ (.x _returnvalue) _returnvalue_2) (+ (.y _returnvalue) _returnvalue_2) (.z _returnvalue)) "0, 0, 0" "1.000000,1.000000,1.000000") "AlwaysSpawn" "MultiplyWithRoot" 0 0))
  (Default|ChangeNumber _returnvalue_3 (Utilities|Text|ToText(Float) Damage "HalfToEven"))
  (if (<= (Variables|Default|GetHealth) 0.0)
    (CallFunction|EnemyDeathSequence)
    (else
      (for _array_element (Actor|GetComponentsByClass "/Script/Engine.StaticMeshComponent")
        (Rendering|Material|SetOverlayMaterial _array_element "/Game/Materials/M_DamageOverlay.M_DamageOverlay" :!class /Script/Engine.MeshComponent))
      (Utilities|FlowControl|Delay 0.1)
      (for _array_element_2 (Actor|GetComponentsByClass "/Script/Engine.StaticMeshComponent")
        (Rendering|Material|SetOverlayMaterial _array_element_2 "/Game/Materials/M_OutlineRed.M_OutlineRed" :!class /Script/Engine.MeshComponent)))))

(event Custom|EnemyDeathSequence
  ;[0.15 0.15 0.15 0.5] Enemy Death Sequence
  (Utilities|FlowControl|Sequence
    (:then_0
      (Game|SpawnActorfromClass "/Game/Particles/BP_EnemyDeathParticle.BP_EnemyDeathParticle_C" (Math|Transform|MakeTransform (Transformation|GetActorLocation) "0, 0, 0" "1.000000,1.000000,1.000000") "AlwaysSpawn" "MultiplyWithRoot" 0 0)
      (Audio|PlaySound2D "/Game/SoundFX/Explosion1.Explosion1" 0.5 (Math|Random|RandomFloatinRange 0.5 1.0) 0.0 0 0)
      (bind _asbp_shmup_hud (Utilities|Casting|CastToBP_ShmupHUD (HUD|GetHUD (Game|GetPlayerController 0))))
      (Default|IncreaseScore (Variables|/Game/Framework/BP_ShmupHUD.BP_ShmupHUD_C|GetUI%20Ref _asbp_shmup_hud) (Variables|Default|GetLootScore)))
    (:then_1
      (Utilities|FlowControl|DelayUntilNextTick)
      (Actor|DestroyActor))))

(event EventBeginPlay
  (for _array_element (Actor|GetComponentsByClass "/Script/Engine.StaticMeshComponent")
    (Rendering|Material|SetOverlayMaterial _array_element "/Game/Materials/M_OutlineRed.M_OutlineRed" :!class /Script/Engine.MeshComponent)))

(fn ConstructionScript)