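; Boss enemy Blueprint for The Anomaly, which loops through teleporting to a random spot and performing a random attack from its pool.
; ChooseNewAttack telegraphs with glow materials and teleport effects, then runs Dash, BulletExplosion or StarPrism, each calling it again when done.
; Unimplemented pool entries fall back to Dash.
; The TurnToFacePlayer timeline eases yaw toward the player, or feeds movement input along NewLocation, reused as a direction, while dashing.
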(event Custom|ChooseNewAttack
  ;[0.1337 0.05471 0.15 0.5] Teleport then Choose Random Attack
  (bind _returnvalue (Actor|GetActorOfClass "/Game/Blueprints/BP_RandomEnemyAimFor.BP_RandomEnemyAimFor_C"))
  (Variables|Default|SetNewLocation (Variables|/Game/Blueprints/BP_RandomEnemyAimFor.BP_RandomEnemyAimFor_C|GetRandomSpot _returnvalue))
  (Rendering|Material|SetMaterial (Variables|Default|GetStaticMesh) 0 "/Game/Materials/M_GlowPurple.M_GlowPurple")
  (Utilities|FlowControl|Delay 0.6)
  (Game|SpawnActorfromClass "/Game/Blueprints/Effects/BP_AnomalyTeleportEffectIn.BP_AnomalyTeleportEffectIn_C" (Math|Transform|MakeTransform (Transformation|GetActorLocation) "0, 0, 0" "1.000000,1.000000,1.000000") "AlwaysSpawn" "MultiplyWithRoot" 0 0)
  (Game|SpawnActorfromClass "/Game/Blueprints/Effects/BP_AnomalyTeleportEffectOut.BP_AnomalyTeleportEffectOut_C" (Math|Transform|MakeTransform (Variables|Default|GetNewLocation) "0, 0, 0" "1.000000,1.000000,1.000000") "AlwaysSpawn" "MultiplyWithRoot" 0 0)
  (Utilities|FlowControl|Delay 0.6)
  (Transformation|SetActorLocation (Variables|Default|GetNewLocation) false true)
  (Utilities|FlowControl|Delay 0.4)
  (Rendering|Material|SetMaterial (Variables|Default|GetStaticMesh) 0 "/Game/Materials/M_GlowRed.M_GlowRed")
  (Utilities|FlowControl|Delay 0.2)
  (switch name (.OutItem (Utilities|Array|Random (Variables|Default|GetAttackPool)))
    (:Default
      (CallFunction|Dash :!label _label))
    (:Dash
      (goto _label))
    (:BulletExplosion
      (CallFunction|BulletExplosion))
    (:StarPrism
      (CallFunction|StarPrism))
    (:BulletRapid
      (goto _label))
    (:BulletBurst
      (goto _label))
    (:CreateCopies
      (goto _label))))

(event Custom|Dash
  (bind _returnvalue (Transformation|GetActorLocation))
  ;[0.15 0.15 0.15 0.5] Dash
  (Game|SpawnActorfromClass "/Game/Blueprints/Effects/BP_AnomalyDashCharge.BP_AnomalyDashCharge_C" (Math|Transform|MakeTransform _returnvalue "0, 0, 0" "1.000000,1.000000,1.000000") "AlwaysSpawn" "MultiplyWithRoot" 0 0)
  (Utilities|FlowControl|Delay 0.6)
  (Variables|Default|SetIsDashing true)
  (Variables|Default|SetNewLocation (Math|Vector|GetUnitDirection(Vector) _returnvalue (Transformation|GetActorLocation (Game|Player|GetPlayerPawn 0))))
  (Utilities|FlowControl|Delay 1.0)
  (Variables|Default|SetIsDashing false)
  (CallFunction|ChooseNewAttack))

(event Custom|BulletExplosion
  ;[0.15 0.15 0.15 0.5] BulletExplosion
  (Variables|Default|SetExplosionCount (Math|Random|RandomIntegerinRange 2 4))
  (Utilities|FlowControl|Delay 0.5 :!label _label)
  (bind _returnvalue (Game|SpawnActorfromClass "/Game/Blueprints/BulletsAndSummons/BP_BulletExplosion.BP_BulletExplosion_C" (Math|Transform|MakeTransform (Transformation|GetActorLocation) "0, 0, 0" "1.000000,1.000000,1.000000") "AlwaysSpawn" "MultiplyWithRoot" 0 0))
  (Variables|/Game/Blueprints/BulletsAndSummons/BP_BulletExplosion.BP_BulletExplosion_C|SetDamageMult _returnvalue 5.0)
  (if (<= (Variables|Default|GetExplosionCount) 0)
    (CallFunction|ChooseNewAttack)
    (else
      (Variables|Default|SetExplosionCount (- (Variables|Default|GetExplosionCount) 1))
      (goto _label))))

(event Custom|StarPrism
  (Game|SpawnActorfromClass "/Game/Blueprints/BulletsAndSummons/BP_EBullet_SpinningStars.BP_EBullet_SpinningStars_C" (Math|Transform|MakeTransform (Transformation|GetActorLocation) "0, 0, 0" "1.000000,1.000000,1.000000") "AlwaysSpawn" "MultiplyWithRoot" 0 0)
  (Utilities|FlowControl|Delay 2.0)
  (CallFunction|ChooseNewAttack))

(event EventOnEnter
  ;[0.06464 0.09486 0.15 0.5] On Enter
  (CallFunction|ChooseNewAttack)
  (Timeline|TurnToFacePlayer Play
    (:Update
      (if (Variables|Default|GetIsDashing)
        (Class|PawnMovementComponent|AddInputVector (Variables|Default|GetFloatingPawnMovement) (Variables|Default|GetNewLocation) false)
        (else
          (Transformation|SetActorRotation (Math|Rotator|MakeRotator 0.0 0.0 (.yaw (Math|Rotator|Lerp(Rotator) (Math|Rotator|MakeRotator 0.0 0.0 (.yaw (Transformation|GetActorRotation))) (Math|Rotator|MakeRotator 0.0 0.0 (.yaw (Math|Rotator|FindLookatRotation (Transformation|GetActorLocation) (Transformation|GetActorLocation (Game|Player|GetPlayerPawn 0))))) 0.15 true)))))))))

(fn ConstructionScript
  (|CallParentFunction))