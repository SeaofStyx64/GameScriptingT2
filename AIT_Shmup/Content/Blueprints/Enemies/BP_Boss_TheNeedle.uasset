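; The Needle boss enemy, a floating pawn that chases the player between randomly chosen attacks.
; On enter, a Cycle timeline drives movement every update, either homing on the player or following a locked dash direction.
; After a delay, it picks from AttackPool: a charged dash, three slower re-aimed dashes, or a trail of spawned saws dropped while chasing.
; Attacks use delays and MaxSpeed changes for wind-up and burst, then chain into the next pick.
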(event Custom|ChooseNewAttack
  (Utilities|FlowControl|Delay 3.0)
  (switch name (.OutItem (Utilities|Array|Random (Variables|Default|GetAttackPool)))
    (:Default
      (CallFunction|Dash :!label _label))
    (:Dash
      (goto _label))
    (:TripleDash
      (CallFunction|TripleDash))
    (:SawDash
      (CallFunction|SawTrail))))

(event Custom|Dash
  ;[0.15 0.15 0.15 0.5] Dash
  (Variables|/Script/Engine.FloatingPawnMovement|SetMaxSpeed (Variables|Default|GetFloatingPawnMovement) 0.0)
  (Game|SpawnActorfromClass "/Game/Blueprints/Effects/BP_NeedleDashCharge.BP_NeedleDashCharge_C" (Math|Transform|MakeTransform (Transformation|GetActorLocation) "0, 0, 0" "1.000000,1.000000,1.000000") "AlwaysSpawn" "MultiplyWithRoot" 0 0)
  (Utilities|FlowControl|Delay 0.6)
  (Variables|Default|SetDashDirection (Math|Vector|GetUnitDirection(Vector) (Transformation|GetActorLocation) (Transformation|GetActorLocation (Game|Player|GetPlayerPawn 0))))
  (Variables|Default|SetIsDashing true)
  (Variables|/Script/Engine.FloatingPawnMovement|SetMaxSpeed (Variables|Default|GetFloatingPawnMovement) 5e+03)
  (Utilities|FlowControl|Delay 0.5)
  (Variables|Default|SetIsDashing false)
  (Variables|/Script/Engine.FloatingPawnMovement|SetMaxSpeed (Variables|Default|GetFloatingPawnMovement) 8e+02)
  (CallFunction|ChooseNewAttack))

(event Custom|TripleDash
  ;[0.15 0.15 0.15 0.5] Triple Dash
  (Variables|Default|SetDashCount 2)
  (Game|SpawnActorfromClass "/Game/Blueprints/Effects/BP_NeedleMiniCharge.BP_NeedleMiniCharge_C" (Math|Transform|MakeTransform (Transformation|GetActorLocation) "0, 0, 0" "1.000000,1.000000,1.000000") "AlwaysSpawn" "MultiplyWithRoot" 0 0)
  (Variables|/Script/Engine.FloatingPawnMovement|SetMaxSpeed (Variables|Default|GetFloatingPawnMovement) 0.0 :!label _label)
  (Utilities|FlowControl|Delay 0.8)
  (Variables|Default|SetDashDirection (Math|Vector|GetUnitDirection(Vector) (Transformation|GetActorLocation) (Transformation|GetActorLocation (Game|Player|GetPlayerPawn 0))))
  (Variables|Default|SetIsDashing true)
  (Variables|/Script/Engine.FloatingPawnMovement|SetMaxSpeed (Variables|Default|GetFloatingPawnMovement) 2.5e+03)
  (Utilities|FlowControl|Delay 0.5)
  (Variables|Default|SetIsDashing false)
  (if (<= (Variables|Default|GetDashCount) 0)
    (Variables|/Script/Engine.FloatingPawnMovement|SetMaxSpeed (Variables|Default|GetFloatingPawnMovement) 8e+02)
    (CallFunction|ChooseNewAttack)
    (else
      (Variables|Default|SetDashCount (- (Variables|Default|GetDashCount) 1))
      (goto _label))))

(event Custom|SawTrail
  ;[0.15 0.15 0.15 0.5] Saws
  (Variables|Default|SetSawCount (Math|Random|RandomIntegerinRange 5 10))
  (Utilities|FlowControl|Delay 0.25 :!label _label)
  (Game|SpawnActorfromClass "/Game/Blueprints/BulletsAndSummons/BP_EBullet_Saw.BP_EBullet_Saw_C" (Math|Transform|MakeTransform (Transformation|GetActorLocation) "0, 0, 0" "1.000000,1.000000,1.000000") "AlwaysSpawn" "MultiplyWithRoot" 0 0)
  (if (<= (Variables|Default|GetSawCount) 0)
    (CallFunction|ChooseNewAttack)
    (else
      (Variables|Default|SetSawCount (- (Variables|Default|GetSawCount) 1))
      (goto _label))))

(event EventOnEnter
  (bind _floatingpawnmovement (Variables|Default|GetFloatingPawnMovement))
  (CallFunction|ChooseNewAttack)
  (Timeline|Cycle Play
    (:Update
      (if (Variables|Default|GetIsDashing)
        (Class|PawnMovementComponent|AddInputVector _floatingpawnmovement (Variables|Default|GetDashDirection) false)
        (else
          (Transformation|SetActorRotation (Math|Rotator|MakeRotator 0.0 0.0 (|RotateToFacePLayer)) true)
          (Class|PawnMovementComponent|AddInputVector _floatingpawnmovement (Math|Vector|GetUnitDirection(Vector) (Transformation|GetActorLocation) (Transformation|GetActorLocation (Game|Player|GetPlayerPawn 0))) false))))))

(fn ConstructionScript
  (|CallParentFunction))