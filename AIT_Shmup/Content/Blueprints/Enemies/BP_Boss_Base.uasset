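; Base boss enemy for the shoot-'em-up, with an outline overlay, health bar widget and timeline-driven swept entrance.
; Capsule overlaps with player bullets or the ship feed ApplyDamage, which rolls the player's crit chance and spawns damage numbers.
; Hits update the bar and flash meshes, restoring the regular enemy outline afterwards.
; Death plays effects, counts the kill, notifies the enemy spawner, drops a weapon pickup and destroys the actor.
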(event OnComponentBeginOverlap(CapsuleHitbox)
  (params (OverlappedComponent :type Primitive%20Component%20Object%20Reference) (OtherActor :type Actor%20Object%20Reference) (OtherComp :type Primitive%20Component%20Object%20Reference) (OtherBodyIndex :type Integer) (bFromSweep :type Boolean) (SweepResult :type Hit%20Result%20Structure%20%28by%20ref%29))
  ;[0.15 0.15 0.15 0.5] On Contact with Player or Player Bullets
  (bind _asbp_base_player_bullet (Utilities|Casting|CastToBP_BasePlayerBullet OtherActor)
    (:then
      (CallFunction|ApplyDamage (Variables|/Game/Blueprints/BulletsAndSummons/BP_BasePlayerBullet.BP_BasePlayerBullet_C|GetDamage _asbp_base_player_bullet)))
    (:CastFailed
      (bind _asbp_player_ship (Utilities|Casting|CastToBP_PlayerShip OtherActor))
      (CallFunction|ApplyDamage (Variables|/Game/Blueprints/PlayerPawns/BP_PlayerShip.BP_PlayerShip_C|GetContactDamage _asbp_player_ship)))))

(event Custom|Apply%20Damage
  (params (Damage :type Float%20%28double-precision%29))
  (bind _returnvalue (Transformation|GetActorLocation))
  (bind _returnvalue_2 (Math|Random|RandomFloatinRange -1e+02 1e+02))
  (bind _returnvalue_3 (Transformation|GetActorLocation))
  (bind _returnvalue_4 (Math|Random|RandomFloatinRange -1e+02 1e+02))
  (bind _returnvalue_5 (* Damage 2.0))
  ;[0.15 0.15 0.15 0.5] Damage Logic
  (bind _asbp_player_ship (Utilities|Casting|CastToBP_PlayerShip (Game|Player|GetPlayerPawn 0)))
  (if (<= (Math|Random|RandomFloatinRange 0.1 1e+02) (Variables|/Game/Blueprints/PlayerPawns/BP_PlayerShip.BP_PlayerShip_C|GetUpgradeCritChance _asbp_player_ship))
    (Variables|Default|SetHealth (- (Variables|Default|GetHealth) _returnvalue_5))
    (Audio|PlaySound2D "/Engine/EditorSounds/GamePreview/PossessPlayer.PossessPlayer" 0.3 1.0 0.0 0 0)
    (bind _returnvalue_6 (Game|SpawnActorfromClass "/Game/Blueprints/Indicators/BP_Indicator_Damage.BP_Indicator_Damage_C" (Math|Transform|MakeTransform (Math|Vector|MakeVector (+ (.x _returnvalue_3) _returnvalue_4) (+ (.y _returnvalue_3) _returnvalue_4) (.z _returnvalue_3)) "0, 0, 0" "1.000000,1.000000,1.000000") "AlwaysSpawn" "MultiplyWithRoot" 0 0))
    (Default|ChangeNumber _returnvalue_6 (Utilities|Text|ToText(Float) _returnvalue_5 "HalfToEven"))
    (Game|SpawnActorfromClass "/Game/Blueprints/Indicators/BP_Indicator_Crit.BP_Indicator_Crit_C" (Math|Transform|MakeTransform (Transformation|GetActorLocation) "0, 0, 0" "1.000000,1.000000,1.000000") "Undefined" "MultiplyWithRoot" 0 0)
    (else
      (Variables|Default|SetHealth (- (Variables|Default|GetHealth) Damage))
      (bind _returnvalue_7 (Game|SpawnActorfromClass "/Game/Blueprints/Indicators/BP_Indicator_Damage.BP_Indicator_Damage_C" (Math|Transform|MakeTransform (Math|Vector|MakeVector (+ (.x _returnvalue) _returnvalue_2) (+ (.y _returnvalue) _returnvalue_2) (.z _returnvalue)) "0, 0, 0" "1.000000,1.000000,1.000000") "AlwaysSpawn" "MultiplyWithRoot" 0 0))
      (Default|ChangeNumber _returnvalue_7 (Utilities|Text|ToText(Float) Damage "HalfToEven"))))
  (Default|SetHealth (Variables|Default|GetBossBarRef) (/ (Variables|Default|GetHealth) (Variables|Default|GetMaxHealth)))
  (if (<= (Variables|Default|GetHealth) 0.0)
    (CallFunction|BossDeathSequence)
    (else
      (for _array_element (Actor|GetComponentsByClass "/Script/Engine.StaticMeshComponent")
        (Rendering|Material|SetOverlayMaterial _array_element "/Game/Materials/M_DamageOverlay.M_DamageOverlay" :!class /Script/Engine.MeshComponent))
      (Utilities|FlowControl|Delay 0.1)
      (for _array_element_2 (Actor|GetComponentsByClass "/Script/Engine.StaticMeshComponent")
        (Rendering|Material|SetOverlayMaterial _array_element_2 "/Game/Materials/M_OutlineEnemy.M_OutlineEnemy" :!class /Script/Engine.MeshComponent)))))

(event Custom|BossDeathSequence
  ;[0.15 0.15 0.15 0.5] Enemy Death Sequence
  (Utilities|FlowControl|Sequence
    (:then_0
      (Game|SpawnActorfromClass "/Game/Particles/BP_EnemyDeathParticle.BP_EnemyDeathParticle_C" (Math|Transform|MakeTransform (Transformation|GetActorLocation) "0, 0, 0" "1.000000,1.000000,1.000000") "AlwaysSpawn" "MultiplyWithRoot" 0 0)
      (Audio|PlaySound2D "/Game/SoundFX/Explosion1.Explosion1" 0.5 (Math|Random|RandomFloatinRange 0.5 1.0) 0.0 0 0))
    (:then_1
      (bind _asbp_shmup_hud (Utilities|Casting|CastToBP_ShmupHUD (HUD|GetHUD (Game|GetPlayerController 0))))
      (Variables|/Game/UI/WBP_StatScreen.WBP_StatScreen_C|SetKillTotal (Variables|/Game/Framework/BP_ShmupHUD.BP_ShmupHUD_C|GetStatScreenRef _asbp_shmup_hud) (+ (Variables|/Game/UI/WBP_StatScreen.WBP_StatScreen_C|GetKillTotal (Variables|/Game/Framework/BP_ShmupHUD.BP_ShmupHUD_C|GetStatScreenRef _asbp_shmup_hud)) 1)))
    (:then_2
      (Default|BossDefeated (Variables|Default|GetBossBarRef))
      (bind _returnvalue (Actor|GetActorOfClass "/Game/Blueprints/BP_EnemySpawner.BP_EnemySpawner_C"))
      (Class|BPISpaceshipFunctions|BossDefeated(Message) _returnvalue)
      (Game|SpawnActorfromClass "/Game/Blueprints/BP_Pickup_Weapon.BP_Pickup_Weapon_C" (Math|Transform|MakeTransform (Transformation|GetActorLocation) "0, 0, 0" "1.000000,1.000000,1.000000") "AlwaysSpawn" "MultiplyWithRoot" 0 0)
      (Utilities|FlowControl|DelayUntilNextTick)
      (Actor|DestroyActor))))

(event EventBeginPlay
  ;[0.15 0.15 0.15 0.5] BeginPlay (Set healthbar, set outline, intro sequence)
  (for _array_element (Actor|GetComponentsByClass "/Script/Engine.StaticMeshComponent")
    (Rendering|Material|SetOverlayMaterial _array_element "/Game/Materials/M_OutlineBoss.M_OutlineBoss" :!class /Script/Engine.MeshComponent)
    (Variables|Default|SetInitialLocation (Transformation|GetActorLocation))
    (bind _returnvalue (UserInterface|CreateWidget "/Game/UI/WBP_BossBar.WBP_BossBar_C"))
    (bind _output_get (Variables|Default|SetBossBarRef _returnvalue))
    (UserInterface|Viewport|AddtoViewport _output_get 0)
    (Default|SetHealth _output_get (Variables|Default|GetMaxHealth))
    (Default|SetName _output_get (Variables|Default|GetBossName))
    (bind _x_offset (Timeline|Timeline PlayFromStart)
      (:Update
        (Transformation|SetActorLocation (+ (Variables|Default|GetInitialLocation) (Math|Vector|MakeVector (* _x_offset -1e+03) 0.0 0.0)) true false)))))

(fn ConstructionScript)