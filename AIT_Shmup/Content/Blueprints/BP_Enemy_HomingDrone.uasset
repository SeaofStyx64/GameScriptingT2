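; BP_Enemy_HomingDrone is an enemy minidrone with a spinning sawblade that homes in on the player.
; Every tick it feeds floating pawn movement the direction toward player controller 0's actor location and sets its yaw to face that point.
; A timeline started on BeginPlay drives the sawblade's relative yaw.
; The GetHitbyPlayer event calls ApplyDamage with a fixed amount.
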(event EventBeginPlay
  ;[0.15 0.15 0.15 0.5] Spinning Sawblade
  (bind _sawspinnew (Timeline|Timeline Play)
    (:Update
      (Transformation|SetRelativeRotation (Variables|Default|GetMinidroneSawblade) (Math|Rotator|MakeRotator 0.0 0.0 _sawspinnew) false false))))

(event EventTick
  (params (DeltaSeconds :type Float%20%28single-precision%29))
  (bind _returnvalue (Transformation|GetActorLocation))
  (bind _returnvalue_2 (Game|GetPlayerController 0))
  (bind _returnvalue_3 (Transformation|GetActorLocation _returnvalue_2))
  (Class|PawnMovementComponent|AddInputVector (Variables|Default|GetFloatingPawnMovement) (Math|Vector|GetUnitDirection(Vector) _returnvalue _returnvalue_3) false)
  (Transformation|SetActorRotation (Math|Rotator|MakeRotator 0.0 0.0 (.yaw (Math|Rotator|FindLookatRotation _returnvalue _returnvalue_3)))))

(event EventGetHitbyPlayer
  (CallFunction|ApplyDamage 1e+02))

(fn ConstructionScript)