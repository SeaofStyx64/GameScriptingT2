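; Player-controlled plane pawn that moves along world axes and fires bullets, with an Enhanced Input context added at BeginPlay.
; Input actions feed FloatingPawnMovement, while Tick interpolates a bank angle from left/right input to roll only the ship model.
; Primary fire switches on BulletType between basic shots alternating left and right spawn points and a three-way spread, using Delays to pace fire.
; Debug keys M and N step BulletType up and down.
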(event Input|EnhancedActionEvents|EnhancedInputActionIA_Forward
  (params (ActionValue :type Boolean) (ElapsedSeconds :type Float%20%28double-precision%29) (TriggeredSeconds :type Float%20%28double-precision%29) (InputAction :type Input%20Action%20Object%20Reference :default "/Game/Data/IA_Forward.IA_Forward"))
  ;[0.15 0.15 0.15 0.5] Movement
  (Class|PawnMovementComponent|AddInputVector (Variables|Default|GetFloatingPawnMovement) "1.000000,0.000000,0.000000" false))

(event Input|EnhancedActionEvents|EnhancedInputActionIA_Right
  (params (ActionValue :type Boolean) (ElapsedSeconds :type Float%20%28double-precision%29) (TriggeredSeconds :type Float%20%28double-precision%29) (InputAction :type Input%20Action%20Object%20Reference :default "/Game/Data/IA_Right.IA_Right"))
  ;[0.15 0.15 0.15 0.5] Movement
  (Class|PawnMovementComponent|AddInputVector (Variables|Default|GetFloatingPawnMovement) "0.000000,1.000000,0.000000" false))

(event Input|EnhancedActionEvents|EnhancedInputActionIA_PrimaryShoot
  (params (ActionValue :type Boolean) (ElapsedSeconds :type Float%20%28double-precision%29) (TriggeredSeconds :type Float%20%28double-precision%29) (InputAction :type Input%20Action%20Object%20Reference :default "/Game/Data/IA_PrimaryShoot.IA_PrimaryShoot"))
  (:Triggered
    (switch int (Variables|Default|GetBulletType)
      (:Default
        ;[0.15 0.15 0.15 0.5] Shoot (basic)
        (Utilities|FlowControl|Delay 0.05 :!label _label)
        (if (Variables|Default|GetShootSwitch)
          (Game|SpawnActorfromClass "/Game/Blueprints/BP_Bullet_Basic.BP_Bullet_Basic_C" (Transformation|GetWorldTransform (Variables|Default|GetFireSpawnPointLeft)) "AlwaysSpawn" "MultiplyWithRoot" 0 0)
          (Variables|Default|SetShootSwitch false)
          (else
            (Game|SpawnActorfromClass "/Game/Blueprints/BP_Bullet_Basic.BP_Bullet_Basic_C" (Transformation|GetWorldTransform (Variables|Default|GetFireSpawnPointRight)) "AlwaysSpawn" "MultiplyWithRoot" 0 0)
            (Variables|Default|SetShootSwitch true))))
      (:0
        (goto _label))
      (:1
        ;[0.15 0.15 0.15 0.5] Shoot (basic)
        (Utilities|FlowControl|Delay 0.2)
        (Game|SpawnActorfromClass "/Game/Blueprints/BP_Bullet_TripleShot.BP_Bullet_TripleShot_C" (Math|Transform|MakeTransform (Transformation|GetActorLocation) "0, 0, 0" "1.000000,1.000000,1.000000") "AlwaysSpawn" "MultiplyWithRoot" 0 0)
        (Game|SpawnActorfromClass "/Game/Blueprints/BP_Bullet_TripleShot.BP_Bullet_TripleShot_C" (Math|Transform|MakeTransform (Transformation|GetActorLocation) "0.000000,20.000000,0.000000" "1.000000,1.000000,1.000000") "AlwaysSpawn" "MultiplyWithRoot" 0 0)
        (Game|SpawnActorfromClass "/Game/Blueprints/BP_Bullet_TripleShot.BP_Bullet_TripleShot_C" (Math|Transform|MakeTransform (Transformation|GetActorLocation) "0.000000,-20.000000,0.000000" "1.000000,1.000000,1.000000") "AlwaysSpawn" "MultiplyWithRoot" 0 0)))))

(event Input|EnhancedActionEvents|EnhancedInputActionIA_Left
  (params (ActionValue :type Boolean) (ElapsedSeconds :type Float%20%28double-precision%29) (TriggeredSeconds :type Float%20%28double-precision%29) (InputAction :type Input%20Action%20Object%20Reference :default "/Game/Data/IA_Left.IA_Left"))
  ;[0.15 0.15 0.15 0.5] Movement
  (Class|PawnMovementComponent|AddInputVector (Variables|Default|GetFloatingPawnMovement) "0.000000,-1.000000,0.000000" false))

(event Input|EnhancedActionEvents|EnhancedInputActionIA_Backwards
  (params (ActionValue :type Boolean) (ElapsedSeconds :type Float%20%28double-precision%29) (TriggeredSeconds :type Float%20%28double-precision%29) (InputAction :type Input%20Action%20Object%20Reference :default "/Game/Data/IA_Backwards.IA_Backwards"))
  ;[0.15 0.15 0.15 0.5] Movement
  (Class|PawnMovementComponent|AddInputVector (Variables|Default|GetFloatingPawnMovement) "-1.000000,0.000000,0.000000" false))

(event EventBeginPlay
  ;[0.15 0.15 0.15 0.5] Add Mapping at Start
  (bind _asplayer_controller (Utilities|Casting|CastToPlayerController (Pawn|GetController)))
  (Input|AddMappingContext (PlayerController|LocalPlayerSubsystems|GetEnhancedInputLocalPlayerSubsystem _asplayer_controller) "/Game/Data/PlayerControlMapping.PlayerControlMapping" 0 "(bIgnoreAllPressedKeysUntilRelease=True,bForceImmediately=False,bNotifyUserSettings=False)"))

(event EventTick
  (params (DeltaSeconds :type Float%20%28single-precision%29))
  (bind _returnvalue (Input|EnhancedActionValues|GetIA_Right))
  (bind _returnvalue_2 (Input|EnhancedActionValues|GetIA_Left))
  (bind _returnvalue_3 (Math|Float|SelectFloat -1.0 0.0 _returnvalue))
  (bind _returnvalue_4 (Math|Float|SelectFloat 1.0 _returnvalue_3 _returnvalue_2))
  ;[0.15 0.15 0.15 0.5] Plane Roll
  (Variables|Default|SetTargetBankAngle _returnvalue_4)
  (Variables|Default|SetCurrentBankAngle (Math|Interpolation|FInterpTo (Variables|Default|GetCurrentBankAngle) _returnvalue_4 DeltaSeconds 8.0))
  (Transformation|SetRelativeRotation (Variables|Default|GetShipModel) (Math|Rotator|MakeRotator (* (Variables|Default|GetMaxBankAngle) (Variables|Default|GetCurrentBankAngle)) 0.0 1.8e+02) false false))

(event Input|KeyboardEvents|DebugKeyM
  (params (Key :type Key%20Structure :default "None") (ActionValue :type Input%20Action%20Value%20Structure))
  (:Pressed
    (Math|Integer|IncrementInt (Variables|Default|GetBulletType))))

(event Input|KeyboardEvents|DebugKeyN
  (params (Key :type Key%20Structure :default "None") (ActionValue :type Input%20Action%20Value%20Structure))
  (:Pressed
    (Math|Integer|DecrementInt (Variables|Default|GetBulletType))))

(fn ConstructionScript)