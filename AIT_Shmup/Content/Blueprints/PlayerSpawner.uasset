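; PlayerSpawner is an actor that brings the player into a shmup by moving on screen, spawning them, then leaving.
; On BeginPlay, an Entrance timeline drives its X position, then it spawns the GameInstance's PlayerClass at its transform and adds the BP_ShmupHUD widget to the viewport.
; An Exit timeline then moves it off screen along X and destroys it.
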(event Custom|LeaveScreen
  (bind _returnvalue (Transformation|GetActorLocation))
  ;[0.15 0.15 0.15 0.5] Go offscreen and despawn
  (bind _leaving (Timeline|Exit PlayFromStart)
    (:Update
      (Transformation|SetActorLocation (Math|Vector|MakeVector _leaving (.y _returnvalue) (.z _returnvalue)) false false))
    (:Finished
      (Actor|DestroyActor))))

(event EventBeginPlay
  (bind _returnvalue (Transformation|GetActorLocation))
  ;[0.15 0.15 0.15 0.5] Move onto screen, spawn player and add HUD
  (bind _entrance (Timeline|Entrance Play)
    (:Update
      (Transformation|SetActorLocation (Math|Vector|MakeVector _entrance (.y _returnvalue) (.z _returnvalue)) false false))
    (:Finished
      (bind _asbp_game_instance (Utilities|Casting|CastToBP_GameInstance (Game|GetGameInstance)))
      (Game|SpawnActorfromClass (Variables|/Game/Framework/BP_GameInstance.BP_GameInstance_C|GetPlayerClass _asbp_game_instance) (Transformation|GetActorTransform) "AlwaysSpawn" "MultiplyWithRoot" 0 0)
      (bind _asbp_shmup_hud (Utilities|Casting|CastToBP_ShmupHUD (HUD|GetHUD (Game|GetPlayerController 0))))
      (UserInterface|Viewport|AddtoViewport (Variables|/Game/Framework/BP_ShmupHUD.BP_ShmupHUD_C|GetUI%20Ref _asbp_shmup_hud) 0)
      (CallFunction|LeaveScreen))))

(fn ConstructionScript)