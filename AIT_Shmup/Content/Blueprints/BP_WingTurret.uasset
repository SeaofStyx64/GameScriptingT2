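; BP_WingTurret is an automatic turret that tracks the nearest enemy and fires bullets on a fixed interval.
; Each tick it gathers all BP_Enemy_Base actors and lerps the TurretHead's relative yaw halfway toward the world look-at yaw of the closest one.
; A looping timer runs ShootAtRandomEnemy, which, despite its name, spawns BP_PTurretBullet at the actor's location using the head's world rotation.
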(event Custom|ShootAtRandomEnemy
  (Game|SpawnActorfromClass "/Game/Blueprints/Bullets/BP_PTurretBullet.BP_PTurretBullet_C" (Math|Transform|MakeTransform (.location (Transformation|GetActorTransform)) (Transformation|GetWorldRotation (Variables|Default|GetTurretHead)) "1.000000,1.000000,1.000000") "AlwaysSpawn" "MultiplyWithRoot" 0 0))

(event EventBeginPlay
  (Utilities|Time|SetTimerbyEvent (delegate Custom|ShootAtRandomEnemy) (Variables|Default|GetFirerateInSeconds) true))

(event EventTick
  (params (DeltaSeconds :type Float%20%28single-precision%29))
  (bind _returnvalue (Transformation|GetActorLocation))
  (bind _turrethead (Variables|Default|GetTurretHead))
  (bind _outactors (Actor|GetAllActorsOfClass "/Game/Blueprints/Enemies/BP_Enemy_Base.BP_Enemy_Base_C"))
  (Transformation|SetRelativeRotation _turrethead (Math|Rotator|MakeRotator 0.0 0.0 (Math|Float|Lerp (.yaw (.rotation (Transformation|GetRelativeTransform _turrethead))) (.yaw (Math|Rotator|FindLookatRotation _returnvalue (Transformation|GetActorLocation (.ReturnValue (Actor|FindNearestActor _returnvalue _outactors))))) 0.5)) false false))

(fn ConstructionScript)