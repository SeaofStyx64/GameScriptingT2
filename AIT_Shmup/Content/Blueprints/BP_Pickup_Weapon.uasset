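; BP_Pickup_Weapon is a weapon pickup actor that homes in on the first player's pawn.
; Each Tick it lerps its rotation toward the look-at yaw to that pawn, then moves along its local forward axis without sweep.
; Both steps use fixed per-frame amounts, so homing speed depends on frame rate.
; This graph holds no pickup or overlap logic, and the construction script only calls the parent.
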(event EventBeginPlay
  (|CallParentFunction) ; This node is disabled and will not be called.\nDrag off pins to build functionality.
)

(event Collision|EventActorBeginOverlap
  (params (OtherActor :type Actor%20Object%20Reference)))

(event EventTick
  (params (DeltaSeconds :type Float%20%28single-precision%29))
  (Transformation|SetActorRotation (Math|Rotator|Lerp(Rotator) (Transformation|GetActorRotation) (Math|Rotator|MakeRotator 0.0 0.0 (.yaw (Math|Rotator|FindLookatRotation (Transformation|GetActorLocation) (Transformation|GetActorLocation (Game|Player|GetPlayerPawn 0))))) 0.15 true))
  (Transformation|AddActorLocalOffset "20.000000,0.000000,0.000000" false false))

(fn ConstructionScript
  (|CallParentFunction))