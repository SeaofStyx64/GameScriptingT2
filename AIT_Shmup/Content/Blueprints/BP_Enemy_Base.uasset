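; BP_Enemy_Base is an enemy actor that takes damage from overlapping bullets and dies at zero health.
; Capsule hitbox overlaps with BP_Bullet subtract its damage from Health and update a health bar widget.
; Surviving hits briefly flash a damage overlay material on all static meshes.
; Death triggers camera shake through the player controller, spawns a particle actor and attached effect, then destroys the enemy next tick.
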(event OnComponentBeginOverlap(CapsuleHitbox)
  (params (OverlappedComponent :type Primitive%20Component%20Object%20Reference) (OtherActor :type Actor%20Object%20Reference) (OtherComp :type Primitive%20Component%20Object%20Reference) (OtherBodyIndex :type Integer) (bFromSweep :type Boolean) (SweepResult :type Hit%20Result%20Structure%20%28by%20ref%29))
  (bind _returnvalue (Transformation|GetActorLocation))
  ;[0.15 0.15 0.15 0.5] Enemy Hit
  (bind _asbp_bullet (Utilities|Casting|CastToBP_Bullet OtherActor))
  (CallFunction|ApplyDamage (Variables|/Game/Blueprints/BP_Bullet.BP_Bullet_C|GetDamage _asbp_bullet))
  (if (<= (Variables|Default|GetHealth) 0.0)
    (Utilities|FlowControl|Sequence
      (:then_0
        (bind _asbp_my_player_controller (Utilities|Casting|CastToBP_MyPlayerController (Game|GetPlayerController 0)))
        (Default|ApplyCameraShake _asbp_my_player_controller))
      (:then_1
        (Game|SpawnActorfromClass "/Game/Particles/BP_EnemyDeathParticle.BP_EnemyDeathParticle_C" (Math|Transform|MakeTransform _returnvalue "0, 0, 0" "1.000000,1.000000,1.000000") "AlwaysSpawn" "MultiplyWithRoot" 0 0)
        (Niagara|SpawnSystemAttached 0 0 "None" _returnvalue "0, 0, 0" "KeepRelativeOffset" false))
      (:then_2
        (Utilities|FlowControl|DelayUntilNextTick)
        (Actor|DestroyActor)))
    (else
      (for _array_element (Actor|GetComponentsByClass "/Script/Engine.StaticMeshComponent")
        (Rendering|Material|SetOverlayMaterial _array_element "/Game/Materials/M_DamageOverlay.M_DamageOverlay" :!class /Script/Engine.MeshComponent))
      (Utilities|FlowControl|Delay 0.2)
      (for _array_element_2 (Actor|GetComponentsByClass "/Script/Engine.StaticMeshComponent")
        (Rendering|Material|SetOverlayMaterial _array_element_2 0 :!class /Script/Engine.MeshComponent)))))

(event Custom|Apply%20Damage
  (params (Damage :type Float%20%28double-precision%29))
  ;[0.15 0.15 0.15 0.5] Enemy Hit
  (Variables|Default|SetHealth (- (Variables|Default|GetHealth) Damage))
  (bind _aswbp_enemy_health_bar (Utilities|Casting|CastToWBP_EnemyHealthBar (UserInterface|GetUserWidgetObject (Variables|Default|GetHealthbar))))
  (Default|SetHealth _aswbp_enemy_health_bar (/ (Variables|Default|GetHealth) (Variables|Default|GetMaxHealth))))

(event EventBeginPlay
  (Variables|Default|SetMaxHealth 3.0))

(event EventTick
  (params (DeltaSeconds :type Float%20%28single-precision%29)))

(fn ConstructionScript)