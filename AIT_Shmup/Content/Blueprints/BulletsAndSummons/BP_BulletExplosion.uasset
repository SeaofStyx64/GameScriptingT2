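; BP_BulletExplosion is a spawner actor that releases a radial burst of BP_EBullet_Basic projectiles.
; Shortly after BeginPlay, a loop spawns the bullets at the SpawnSpot location, stepping SpawnRotation's yaw in equal increments to form a full ring.
; Each bullet spawns regardless of collision and then has its Damage scaled by DamageMult.
; The actor has no logic to destroy itself after the burst.
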(event EventBeginPlay
  (Utilities|FlowControl|Delay 0.1)
  (for _index (range 0 15)
    (bind _returnvalue (Game|SpawnActorfromClass "/Game/Blueprints/BulletsAndSummons/BP_EBullet_Basic.BP_EBullet_Basic_C" (Math|Transform|MakeTransform (Transformation|GetWorldLocation (Variables|Default|GetSpawnSpot)) (Variables|Default|GetSpawnRotation) "1.000000,1.000000,1.000000") "AlwaysSpawn" "MultiplyWithRoot" 0 0))
    (Variables|/Game/Blueprints/BulletsAndSummons/BP_BaseEnemyBullet.BP_BaseEnemyBullet_C|SetDamage _returnvalue (* (Variables|/Game/Blueprints/BulletsAndSummons/BP_BaseEnemyBullet.BP_BaseEnemyBullet_C|GetDamage _returnvalue) (Variables|Default|GetDamageMult)))
    (Variables|Default|SetSpawnRotation (Math|Rotator|MakeRotator 0.0 0.0 (+ (.yaw (Variables|Default|GetSpawnRotation)) 22.5)))))

(fn ConstructionScript)