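; BP_PBullet_Star is a homing star projectile that survives a limited number of overlaps before destroying itself.
; It disables ProjectileMovement and moves forward a fixed step each Tick, lerping its yaw toward the nearest HomingTarget-tagged actor, so speed and turning are frame-rate dependent.
; The StarStuff timeline spins and scales the Star component for the spin and decay visuals.
; Each overlap decrements HitsTillDestroy; once exhausted, the next overlap destroys it a tick later.
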(event EventBeginPlay
  (bind _star (Variables|Default|GetStar))
  ;[0.15 0.15 0.15 0.5] Change in rotation (for spin visual effect) and change in shape (for decay visual effect)
  (|CallParentFunction)
  (Components|Activation|SetActive (Variables|Default|GetProjectileMovement) false false)
  (bind (_direction _spin _size) (Timeline|StarStuff Play)
    (:Update
      (Transformation|SetWorldRotation _star (Math|Rotator|MakeRotator 0.0 0.0 _spin) false false)
      (Transformation|SetWorldScale3D _star (Math|Vector|MakeVector _size _size _size)))))

(event EventTick
  (params (DeltaSeconds :type Float%20%28single-precision%29))
  (bind _returnvalue (Transformation|GetActorLocation))
  ;[0.15 0.15 0.15 0.5] Home for targets
  (bind _outactors (Actor|GetAllActorswithTag "HomingTarget"))
  (Transformation|SetActorRotation (Math|Rotator|MakeRotator 0.0 0.0 (.yaw (Math|Rotator|Lerp(Rotator) (Math|Rotator|MakeRotator 0.0 0.0 (.yaw (Transformation|GetActorRotation))) (Math|Rotator|MakeRotator 0.0 0.0 (.yaw (Math|Rotator|FindLookatRotation _returnvalue (Transformation|GetActorLocation (.ReturnValue (Actor|FindNearestActor _returnvalue _outactors)))))) 0.15 true))))
  (Transformation|AddActorLocalOffset "40.000000,0.000000,0.000000" false false))

(event Collision|EventActorBeginOverlap
  (params (OtherActor :type Actor%20Object%20Reference))
  (if (<= (Variables|Default|GetHitsTillDestroy) 0)
    (Utilities|FlowControl|DelayUntilNextTick)
    (Actor|DestroyActor)
    (else
      (Variables|Default|SetHitsTillDestroy (- (Variables|Default|GetHitsTillDestroy) 1)))))

(fn ConstructionScript
  (|CallParentFunction))