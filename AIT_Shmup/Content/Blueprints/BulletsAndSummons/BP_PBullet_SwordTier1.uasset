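; BP_PBullet_SwordTier1 is a tier 1 sword attack built as a bullet actor that swings a blade instead of flying.
; On BeginPlay it runs the parent logic, deactivates ProjectileMovement and plays the Bladeswing timeline.
; The timeline drives the Blade component's relative yaw and scale, then destroys the actor when it finishes.
; It defines no overlap or hit logic of its own.
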(event EventBeginPlay
  (bind _blade (Variables|Default|GetBlade))
  (|CallParentFunction)
  (Components|Activation|SetActive (Variables|Default|GetProjectileMovement) false false)
  (bind (_direction _bladeswing _size) (Timeline|Bladeswing Play)
    (:Update
      (Transformation|SetRelativeRotation _blade (Math|Rotator|MakeRotator 0.0 0.0 _bladeswing) false false)
      (Transformation|SetRelativeScale3D _blade _size))
    (:Finished
      (Actor|DestroyActor))))

(event Collision|EventActorBeginOverlap
  (params (OtherActor :type Actor%20Object%20Reference)))

(event EventTick
  (params (DeltaSeconds :type Float%20%28single-precision%29))
  (|CallParentFunction DeltaSeconds) ; This node is disabled and will not be called.\nDrag off pins to build functionality.
)

(fn ConstructionScript
  (|CallParentFunction))