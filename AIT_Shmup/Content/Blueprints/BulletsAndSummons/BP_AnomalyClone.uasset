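; BP_AnomalyClone is a summoned clone actor that constantly faces the player and vanishes when touched.
; Tick turns it toward player pawn 0, and BeginPlay switches its mesh to a white glow material after a short delay.
; Overlap with the player ship or a player bullet applies a dodge overlay material, then destroys the clone moments later, with no damage dealt in this graph.
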(event EventBeginPlay
  (Utilities|FlowControl|Delay 0.4)
  (Rendering|Material|SetMaterial (Variables|Default|GetStaticMesh) 0 "/Game/Materials/M_GlowWhite.M_GlowWhite"))

(event Collision|EventActorBeginOverlap
  (params (OtherActor :type Actor%20Object%20Reference))
  (Utilities|Casting|CastToBP_PlayerShip OtherActor
    (:then
      _)
    (:CastFailed
      (Utilities|Casting|CastToBP_BasePlayerBullet OtherActor)))
  (Rendering|Material|SetOverlayMaterial (Variables|Default|GetStaticMesh) "/Game/Materials/M_DodgeOverlay.M_DodgeOverlay" :!class /Script/Engine.MeshComponent)
  (Utilities|FlowControl|Delay 0.2)
  (Actor|DestroyActor))

(event EventTick
  (params (DeltaSeconds :type Float%20%28single-precision%29))
  (Transformation|SetActorRotation (Math|Rotator|FindLookatRotation (Transformation|GetActorLocation) (Transformation|GetActorLocation (Game|Player|GetPlayerPawn 0)))))

(fn ConstructionScript)