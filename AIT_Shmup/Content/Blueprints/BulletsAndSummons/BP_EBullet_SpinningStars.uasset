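; Enemy bullet Blueprint for a spinning-stars hazard that stays off projectile movement and destroys itself when its Lifetime timeline ends.
; On BeginPlay it runs the parent logic, deactivates ProjectileMovement and plays the timeline.
; The Distance track scales PivotCentre in X and Y, while StarSize sets the world scale of Saw1 and Saw2, keeping star size independent of the pivot's scale.
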(event EventBeginPlay
  (|CallParentFunction)
  (Components|Activation|SetActive (Variables|Default|GetProjectileMovement) false false)
  (bind (_direction _distance _starsize) (Timeline|Lifetime Play)
    (:Update
      (Transformation|SetRelativeScale3D (Variables|Default|GetPivotCentre) (Math|Vector|MakeVector _distance _distance 0.0))
      (Transformation|SetWorldScale3D (Variables|Default|GetSaw1) (Math|Vector|MakeVector _starsize _starsize _starsize)))
    (:Finished
      (Actor|DestroyActor))))

(event EventTick
  (params (DeltaSeconds :type Float%20%28single-precision%29))
  (|CallParentFunction DeltaSeconds) ; This node is disabled and will not be called.\nDrag off pins to build functionality.
)

(fn ConstructionScript
  (|CallParentFunction))