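; Tier 3 sword attack built as a player bullet that performs a two-blade swing in place of flying.
; On BeginPlay it runs the parent logic, deactivates projectile movement and plays the BladesSwing timeline.
; The timeline drives a separate yaw for each blade and a shared scale for both, then destroys the actor when finished.
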(event EventBeginPlay
  (bind _blade2 (Variables|Default|GetBlade2))
  (|CallParentFunction)
  (Components|Activation|SetActive (Variables|Default|GetProjectileMovement) false false)
  (bind (_direction _bladeswing _bladeswing2 _size) (Timeline|BladesSwing Play)
    (:Update
      (Transformation|SetRelativeRotation (Variables|Default|GetBlade1) (Math|Rotator|MakeRotator 0.0 0.0 _bladeswing) false false)
      (Transformation|SetRelativeRotation _blade2 (Math|Rotator|MakeRotator 0.0 0.0 _bladeswing2) false false)
      (Transformation|SetRelativeScale3D _blade2 _size))
    (:Finished
      (Actor|DestroyActor))))

(event Collision|EventActorBeginOverlap
  (params (OtherActor :type Actor%20Object%20Reference)))

(event EventTick
  (params (DeltaSeconds :type Float%20%28single-precision%29))
  (|CallParentFunction DeltaSeconds) ; This node is disabled and will not be called.\nDrag off pins to build functionality.
)

(fn ConstructionScript
  (|CallParentFunction))