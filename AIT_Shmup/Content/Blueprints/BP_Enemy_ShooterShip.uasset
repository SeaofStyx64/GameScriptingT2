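; BP_Enemy_ShooterShip is an enemy ship that flies in, stops, then fires at the player.
; On BeginPlay it waits a random delay, deactivates its projectile movement, fires once and starts a looping timer with a randomized interval to spawn BP_Bullet_Enemy at BulletSpawnPoint.
; A Timeline, started after the first shot, turns the ship toward the player pawn on each update.
; GetHitbyPlayer applies fixed damage to the ship.
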(event Custom|ShootBullet
  (Game|SpawnActorfromClass "/Game/Blueprints/BP_Bullet_Enemy.BP_Bullet_Enemy_C" (Transformation|GetWorldTransform (Variables|Default|GetBulletSpawnPoint)) "Undefined" "MultiplyWithRoot" 0 0))

(event EventBeginPlay
  (Utilities|FlowControl|Delay (Math|Random|RandomFloatinRange 2.0 4.0))
  (Components|Activation|Deactivate (Variables|Default|GetProjectileMovement))
  (CallFunction|ShootBullet)
  (bind _returnvalue (Utilities|Time|SetTimerbyEvent (delegate Custom|ShootBullet) (Math|Random|RandomFloatinRange 1.0 3.0) true true))
  (Variables|Default|SetShootTimer _returnvalue)
  (Timeline|Timeline PlayFromStart
    (:Update
      (Transformation|SetActorRotation (Math|Rotator|FindLookatRotation (Transformation|GetWorldLocation (Variables|Default|GetDefaultSceneRoot)) (Transformation|GetActorLocation (Game|Player|GetPlayerPawn 0)))))))

(event EventGetHitbyPlayer
  (CallFunction|ApplyDamage 1e+02))

(fn ConstructionScript)